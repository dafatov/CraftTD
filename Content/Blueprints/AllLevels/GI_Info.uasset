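; GI_Info is the Game Instance that runs multiplayer session flow and menu display for the game.
; It hosts listen-server sessions on GameBoard with name and player count as extra settings, reads the count back on join, and prints failures in red.
; Show events create widgets, mostly cached; craft and help menus fill from tower recipes and input mappings.
; It also toggles player input and cursor for menus and spawns an overhead camera.
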(event Custom|ShowEscapeMenu
  (bind _returnvalue (Game|GetPlayerCharacter 0))
  ;[1 1 1] Show EscapeMenu
  (if (Variables|ClientValues|GetisGame?)
    (Viewport|RemoveAllWidgets :!label _label)
    (Utilities|IsValid (Variables|Widgets|GetEscapeMenu)
      (:Is%20Valid
        _)
      (:Is%20Not%20Valid
        (bind _returnvalue_2 (UserInterface|CreateWidget "/Game/Blueprints/UI/AllLevels/WB_EscapeMenu.WB_EscapeMenu_C"))
        (Variables|Widgets|SetEscapeMenu _returnvalue_2)))
    (UserInterface|Viewport|AddtoViewport (Variables|Widgets|GetEscapeMenu) 0)
    (Input|DisableInput _returnvalue (Game|GetPlayerController 0))
    (bind _asbp_player_character (Utilities|Casting|CastToBP_PlayerCharacter _returnvalue))
    (Default|SetShownCursor _asbp_player_character true)
    (else
      (bind _returnvalue_3 (Game|GetCurrentLevelName true))
      (if (Utilities|Enum|Equal(Enum) _returnvalue_3 "GameBoard")
        (goto _label)))))

(event Custom|ShowHostMenu
  ;[1 1 1] Show HostMenu
  (Utilities|IsValid (Variables|Widgets|GetHostMenu)
    (:Is%20Valid
      _)
    (:Is%20Not%20Valid
      (bind _returnvalue (UserInterface|CreateWidget "/Game/Blueprints/UI/MainMenu/WB_HostMenu.WB_HostMenu_C" (Game|GetPlayerController 0)))
      (Variables|Widgets|SetHostMenu _returnvalue)))
  (UserInterface|Viewport|AddtoViewport (Variables|Widgets|GetHostMenu) 0))

(event Custom|ShowGameResultMenu
  (params (IsWin? :type Boolean))
  ;[1 1 1] ShowGameResultMenu
  (bind _returnvalue (UserInterface|CreateWidget "/Game/Blueprints/UI/AllLevels/WB_GameResult.WB_GameResult_C" (Game|GetPlayerController 0) IsWin?))
  (Viewport|RemoveAllWidgets)
  (UserInterface|Viewport|AddtoViewport _returnvalue 0))

(event Custom|SpawnCameraActor&Set
  ;[1 1 1] CreateCameraUp
  (bind _asbp_player_character (Utilities|Casting|CastToBP_PlayerCharacter (Game|GetPlayerCharacter 0)))
  (Variables|/Game/Blueprints/Player/BP_PlayerCharacter.BP_PlayerCharacter_C|GetCameraUp _asbp_player_character
    (:then)
    (:else
      (bind _returnvalue (Game|SpawnActorfromClass "/Script/Engine.CameraActor" (Math|Transform|MakeTransform "0.000000,3100.000000,3200.000000" "-55.000000, 0, 0" "1,1,1") "Undefined" 0 0))
      (bind _output_get (Variables|/Game/Blueprints/Player/BP_PlayerCharacter.BP_PlayerCharacter_C|SetCameraUp _asbp_player_character _returnvalue))
      (Camera|SetFieldOfView (Variables|/Script/Engine.CameraActor|GetCameraComponent _output_get) 1.2e+02))))

(event Custom|ShowCraftMenu
  (bind _returnvalue (Game|GetPlayerCharacter 0))
  (bind _returnvalue_2 (Game|GetPlayerController 0))
  (bind _actionmenu (Variables|Widgets|GetActionMenu))
  ;[1 1 1] ShowCraftMenu
  (Utilities|IsValid (Variables|Widgets|GetCraftMenu)
    (:Is%20Valid
      _)
    (:Is%20Not%20Valid
      (bind _returnvalue_3 (UserInterface|CreateWidget "/Game/Blueprints/UI/AllLevels/WB_CraftViewMenu.WB_CraftViewMenu_C" _returnvalue_2))
      (bind _output_get (Variables|Widgets|SetCraftMenu _returnvalue_3))
      (CallFunction|GetAllCraft&AddtoWB)))
  (UserInterface|Viewport|AddtoViewport _output_get 2)
  (Widget|SetIsEnabled (Variables|/Game/Blueprints/UI/AllLevels/WB_ActionMenu.WB_ActionMenu_C|GetCraftMenu (Variables|Widgets|GetActionMenu)) false)
  (Input|DisableInput _returnvalue _returnvalue_2)
  (bind _asbp_player_character (Utilities|Casting|CastToBP_PlayerCharacter _returnvalue))
  (Default|SetShownCursor _asbp_player_character true)
  (Variables|ClientValues|SetActionMode "NewEnumerator0")
  (Default|SetCraftUnselected _actionmenu)
  (Default|SetBuildUnselected _actionmenu)
  (Default|SetDestroyUnselected _actionmenu))

(event Custom|ShowHelpMenu
  (bind _returnvalue (Game|GetPlayerCharacter 0))
  (bind _returnvalue_2 (Game|GetPlayerController 0))
  (bind _actionmenu (Variables|Widgets|GetActionMenu))
  ;[1 1 1] ShowHelpMenu
  (Utilities|IsValid (Variables|Widgets|GetHelpMenu)
    (:Is%20Valid
      _)
    (:Is%20Not%20Valid
      (bind _returnvalue_3 (UserInterface|CreateWidget "/Game/Blueprints/UI/AllLevels/WB_HelpMenu.WB_HelpMenu_C" _returnvalue_2))
      (bind _output_get (Variables|Widgets|SetHelpMenu _returnvalue_3))
      (CallFunction|GetInputs&AddtoWB)))
  (UserInterface|Viewport|AddtoViewport _output_get 2)
  (Input|DisableInput _returnvalue _returnvalue_2)
  (bind _asbp_player_character (Utilities|Casting|CastToBP_PlayerCharacter _returnvalue))
  (Default|SetShownCursor _asbp_player_character true)
  (Variables|ClientValues|SetActionMode "NewEnumerator0")
  (Default|SetCraftUnselected _actionmenu)
  (Default|SetBuildUnselected _actionmenu)
  (Default|SetDestroyUnselected _actionmenu))

(event Custom|ShowMainMenu
  ;[1 1 1] Show MainMenu
  (Utilities|IsValid (Variables|Widgets|GetMainMenu)
    (:Is%20Valid
      _)
    (:Is%20Not%20Valid
      (bind _returnvalue (UserInterface|CreateWidget "/Game/Blueprints/UI/MainMenu/WB_MainMenu.WB_MainMenu_C" (Game|GetPlayerController 0)))
      (Variables|Widgets|SetMainMenu _returnvalue)))
  (UserInterface|Viewport|AddtoViewport (Variables|Widgets|GetMainMenu) 0))

(event Custom|ShowActionMenu
  ;[1 1 1] ShowActionMenu
  (Utilities|IsValid (Variables|Widgets|GetActionMenu)
    (:Is%20Valid
      _)
    (:Is%20Not%20Valid
      (bind _returnvalue (UserInterface|CreateWidget "/Game/Blueprints/UI/AllLevels/WB_ActionMenu.WB_ActionMenu_C" (Game|GetPlayerController 0)))
      (Variables|Widgets|SetActionMenu _returnvalue)))
  (if (not (UserInterface|Viewport|IsinViewport (Variables|Widgets|GetActionMenu)))
    (UserInterface|Viewport|AddtoViewport (Variables|Widgets|GetActionMenu) 0)))

(event Custom|ShowServerMenu
  ;[1 1 1] Show ServerMenu
  (bind _returnvalue (UserInterface|CreateWidget "/Game/Blueprints/UI/MainMenu/WB_ServerMenu.WB_ServerMenu_C" (Game|GetPlayerController 0)))
  (UserInterface|Viewport|AddtoViewport _returnvalue 0))

(event Custom|ShowOptionsMenu
  (params (IsFromEscapeMenu? :type Boolean))
  ;[1 1 1] Show OptionMenu
  (Utilities|IsValid (Variables|Widgets|GetOptionsMenu)
    (:Is%20Valid
      _)
    (:Is%20Not%20Valid
      (bind _returnvalue (UserInterface|CreateWidget "/Game/Blueprints/UI/MainMenu/WB_OptionsMenu.WB_OptionsMenu_C" (Game|GetPlayerController 0)))
      (bind _output_get (Variables|Widgets|SetOptionsMenu _returnvalue))))
  (UserInterface|Viewport|AddtoViewport (Variables|Widgets|GetOptionsMenu) 0)
  (Variables|/Game/Blueprints/UI/MainMenu/WB_OptionsMenu.WB_OptionsMenu_C|SetIsFromEscapeMenu? _output_get IsFromEscapeMenu?))

(event Custom|LaunchGame
  (params (NumberOfPlayers :type Integer) (EnableLAN? :type Boolean) (ServerName :type Text))
  ;[1 1 1] Host Server & launch
  (bind _output_get (Variables|ServerValues|SetNumberOfPlayers NumberOfPlayers))
  (CallFunction|ShowLoadingScreen)
  (|AdvancedSession (Utilities|Array|MakeArray (Class|AdvancedSessionsLibrary|MakeLiteralSessionPropertyString "Name" (Utilities|String|ToString(Text) ServerName)) (Class|AdvancedSessionsLibrary|MakeLiteralSessionPropertyInt "NumberOfPlayers" _output_get)) (Game|GetPlayerController 0) _output_get 0 EnableLAN? true false true true false false false true
    (:OnSuccess
      (Game|OpenLevel(byName) "GameBoard" true "listen")
      (Utilities|GameStart))
    (:OnFailure
      (Utilities|DisplayErrorMessage "Failed To Create Session"))))

(event Custom|ShowLoadingScreen
  ;[1 1 1] Show LoadingScreen
  (Utilities|IsValid (Variables|Widgets|GetLoadingScreen)
    (:Is%20Valid
      _)
    (:Is%20Not%20Valid
      (bind _returnvalue (UserInterface|CreateWidget "/Game/Blueprints/UI/AllLevels/WB_LoadingScreen.WB_LoadingScreen_C" (Game|GetPlayerController 0)))
      (Variables|Widgets|SetLoadingScreen _returnvalue)))
  (UserInterface|Viewport|AddtoViewport (Variables|Widgets|GetLoadingScreen) 0))

(event Custom|JoinServer
  (params (SessionToJoin :type Blueprint%20Session%20Result%20Structure))
  ;[1 1 1] Join Server
  (CallFunction|ShowLoadingScreen)
  (|JoinSession (Game|GetPlayerController 0) SessionToJoin
    (:OnSuccess
      (Utilities|GameStart
        (:Out
          (Utilities|LoadJoinData SessionToJoin))))
    (:OnFailure
      (Utilities|DisplayErrorMessage "Failed To Join Session"))))

(event Custom|DestroySessionCaller
  (params (PlayerController :type Player%20Controller%20Object%20Reference))
  ;[1 1 1] Leave from game
  (|DestroySession PlayerController
    (:OnSuccess
      (Game|OpenLevel(byName) "MainMenu")
      (CallFunction|ShowMainMenu)
      (Variables|ClientValues|SetisGame? false))))

(event EventHandleNetworkError
  (params (FailureType :type ENetworkFailure%20Enum :default "NetDriverAlreadyExists") (bIsServer :type Boolean))
  ;[1 1 1] Error handlers
  (if (not bIsServer)
    (Utilities|DisplayErrorMessage (CallFunction|NetErrortoString FailureType))))

(event EventHandleTravelError
  (params (FailureType :type ETravelFailure%20Enum :default "NoLevel"))
  ;[1 1 1] Error handlers
  (bind _error (CallFunction|TravelErrortoString FailureType))
  (Utilities|DisplayErrorMessage _error))

(event EventInit
  ;[1 1 1] Временный костыль
  (Utilities|FlowControl|Delay 1.0)
  (bind _asbp_player_character (Utilities|Casting|CastToBP_PlayerCharacter (Game|GetPlayerCharacter 0)))
  (if (Variables|/Game/Blueprints/Player/BP_PlayerCharacter.BP_PlayerCharacter_C|GetDebug? _asbp_player_character)
    _))

(fn NetErrortoString
  (params (FailureType :type ENetworkFailure%20Enum :default "NetDriverAlreadyExists"))
  (return (Utilities|String|EnumtoString FailureType)))

(fn TravelErrortoString
  (params (FailureType :type ETravelFailure%20Enum :default "NoLevel"))
  (return (Utilities|String|EnumtoString FailureType)))

(fn GetAllCraft&AddtoWB
  (bind _asbp_player_character (Utilities|Casting|CastToBP_PlayerCharacter (Game|GetPlayerCharacter 0)))
  (for _array_element (Variables|/Game/Blueprints/Player/BP_PlayerCharacter.BP_PlayerCharacter_C|GetAllTowerRecipes _asbp_player_character)
    (bind _returnvalue (UserInterface|CreateWidget "/Game/Blueprints/UI/AllLevels/WB_CraftViewElement.WB_CraftViewElement_C" (Game|GetPlayerController 0) _array_element))
    (Widget|Panel|AddChild (Variables|/Game/Blueprints/UI/AllLevels/WB_CraftViewMenu.WB_CraftViewMenu_C|GetWrapBox_0 (Variables|Widgets|GetCraftMenu)) _returnvalue)))

(fn GetInputs&AddtoWB
  (bind _returnvalue (Class|InputSettings|GetInputSettings))
  (for _array_element (Class|InputSettings|GetActionNames _returnvalue)
    (bind _returnvalue_2 (UserInterface|CreateWidget "/Game/Blueprints/UI/AllLevels/WB_InputElement.WB_InputElement_C" 0 (Utilities|Array|Get(acopy) (Class|InputSettings|GetActionMappingbyName _returnvalue _array_element))))
    (Widget|Panel|AddChild (Variables|/Game/Blueprints/UI/AllLevels/WB_HelpMenu.WB_HelpMenu_C|GetControlList (Variables|Widgets|GetHelpMenu)) _returnvalue_2)))