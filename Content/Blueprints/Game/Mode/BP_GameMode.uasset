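; BP_GameMode is the game mode for a multiplayer, wave-based tower defense with building.
; On login it registers each player controller and, after a short delay, has the character set a unique color and starting build counter from the player list.
; WaveFinish resets tower idle-shot bonuses, spawner wave flags and the ready count, then refreshes build counters through player character 0.
; That character also announces game end once the first spawner's wave index exceeds its maximum.
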(event Custom|WaveFinish
  (Utilities|Casting|CastToGI_Info (Game|GetGameInstance))
  (bind _outactors (Actor|GetAllActorsOfClass "/Game/Blueprints/Map/BP_Tower.BP_Tower_C"))
  (for _array_element _outactors
    (Default|IdleShotStopTimer _array_element)
    (Variables|/Game/Blueprints/Map/BP_Tower.BP_Tower_C|SetIdleShotAddDamage _array_element 0.0))
  (bind _outactors_2 (Actor|GetAllActorsOfClass "/Game/Blueprints/Map/BP_Spawner.BP_Spawner_C"))
  (for _array_element_2 _outactors_2
    (Variables|/Game/Blueprints/Map/BP_Spawner.BP_Spawner_C|SetIsWave? _array_element_2 false))
  (bind _asbp_player_character (Utilities|Casting|CastToBP_PlayerCharacter (Game|GetPlayerCharacter 0)))
  (Default|Action:WaveFinish-Server _asbp_player_character)
  (bind _asbp_player_character_2 (Utilities|Casting|CastToBP_PlayerCharacter (Game|GetPlayerCharacter 0)))
  (Default|SetStartRemainBuildsCounter _asbp_player_character_2 (Variables|Default|GetRegisteredPlayers))
  (Variables|Default|SetReadyPlayersCounter 0)
  (if (> (Variables|/Game/Blueprints/Map/BP_Spawner.BP_Spawner_C|GetCurrentWaveIndex (Utilities|Array|Get(acopy) _outactors_2)) (Variables|/Game/Blueprints/Map/BP_Spawner.BP_Spawner_C|GetMaxWaves (Utilities|Array|Get(acopy) _outactors_2)))
    (Default|GameFinish:DisableandAnnounce _asbp_player_character_2 true)))

(event EventPostLogin
  (params (NewPlayer :type Player%20Controller%20Object%20Reference))
  (bind _registeredplayers (Variables|Default|GetRegisteredPlayers))
  (bind _asbp_player_controller (Utilities|Casting|CastToBP_PlayerController NewPlayer))
  (Utilities|Array|AddUnique (Variables|Default|GetRegisteredPlayers) _asbp_player_controller)
  (Utilities|FlowControl|Delay 1.0)
  (bind _asbp_player_character (Utilities|Casting|CastToBP_PlayerCharacter (Pawn|GetControlledPawn _asbp_player_controller)))
  (Default|SetUniquePlayerColor _asbp_player_character _registeredplayers)
  (Default|SetStartRemainBuildsCounter _asbp_player_character _registeredplayers))

(fn ConstructionScript)