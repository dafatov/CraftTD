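; BP_PlayerStart is a map actor for the player start area, with three teleport triggers that move overlapping player characters on the server.
; Teleport and Teleport1 shift the character by a fixed offset in opposite world Y directions, the latter with a slight lift.
; Teleport2 waits until the GameMode's registered players reach the GameInstance's player count.
; It then moves the character to the first BP_Spawner's portal Spawn socket and calls AfterTeleport with that socket's rotation.
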(event OnComponentBeginOverlap(Teleport1)
  (params (OverlappedComponent :type Primitive%20Component%20Object%20Reference) (OtherActor :type Actor%20Object%20Reference) (OtherComp :type Primitive%20Component%20Object%20Reference) (OtherBodyIndex :type Integer) (bFromSweep :type Boolean) (SweepResult :type Hit%20Result%20Structure%20%28by%20ref%29))
  (Networking|SwitchHasAuthority
    (:Authority
      (bind _asbp_player_character (Utilities|Casting|CastToBP_PlayerCharacter OtherActor))
      (Transformation|AddWorldOffset (Variables|/Script/Engine.Actor|GetRootComponent _asbp_player_character) (* "0,-1.000000,0.030000" 300) false true))))

(event OnComponentBeginOverlap(Teleport)
  (params (OverlappedComponent :type Primitive%20Component%20Object%20Reference) (OtherActor :type Actor%20Object%20Reference) (OtherComp :type Primitive%20Component%20Object%20Reference) (OtherBodyIndex :type Integer) (bFromSweep :type Boolean) (SweepResult :type Hit%20Result%20Structure%20%28by%20ref%29))
  (Networking|SwitchHasAuthority
    (:Authority
      (bind _asbp_player_character (Utilities|Casting|CastToBP_PlayerCharacter OtherActor))
      (Transformation|AddWorldOffset (Variables|/Script/Engine.Actor|GetRootComponent _asbp_player_character) (* "0,1.000000,0.000000" 300) false true))))

(event OnComponentBeginOverlap(Teleport2)
  (params (OverlappedComponent :type Primitive%20Component%20Object%20Reference) (OtherActor :type Actor%20Object%20Reference) (OtherComp :type Primitive%20Component%20Object%20Reference) (OtherBodyIndex :type Integer) (bFromSweep :type Boolean) (SweepResult :type Hit%20Result%20Structure%20%28by%20ref%29))
  (Networking|SwitchHasAuthority
    (:Authority
      (bind _asbp_player_character (Utilities|Casting|CastToBP_PlayerCharacter OtherActor))
      (if (>= (Utilities|Array|Length (Variables|/Game/Blueprints/Game/Mode/BP_GameMode.BP_GameMode_C|GetRegisteredPlayers (Variables|Default|GetGameModeRef))) (Variables|/Game/Blueprints/AllLevels/GI_Info.GI_Info_C|GetNumberOfPlayers (Variables|Default|GetGameInstanceRef)))
        (bind _outactors (Actor|GetAllActorsOfClass "/Game/Blueprints/Map/BP_Spawner.BP_Spawner_C"))
        (Transformation|SetWorldLocation (Variables|/Script/Engine.Character|GetCapsuleComponent _asbp_player_character) (Transformation|GetSocketLocation (Variables|/Game/Blueprints/Map/BP_Spawner.BP_Spawner_C|GetPortal (Utilities|Array|Get(acopy) _outactors)) "Spawn") false true)
        (Default|AfterTeleport _asbp_player_character (Transformation|GetSocketRotation (Variables|/Game/Blueprints/Map/BP_Spawner.BP_Spawner_C|GetPortal (Utilities|Array|Get(acopy) _outactors)) "Spawn"))))))

(event EventBeginPlay
  (bind _asgi_info (Utilities|Casting|CastToGI_Info (Game|GetGameInstance)))
  (Variables|Default|SetGameInstanceRef _asgi_info)
  (bind _asbp_game_mode (Utilities|Casting|CastToBP_GameMode (Game|GetGameMode)))
  (Variables|Default|SetGameModeRef _asbp_game_mode))

(event Collision|EventActorBeginOverlap
  (params (OtherActor :type Actor%20Object%20Reference)))

(event EventTick
  (params (DeltaSeconds :type Float%20%28single-precision%29)))

(fn ConstructionScript)