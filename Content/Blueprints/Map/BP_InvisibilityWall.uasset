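; BP_InvisibilityWall is an invisible-wall actor that sends the player back to a spawn portal on contact.
; When its Box is hit by a BP_PlayerCharacter, it teleports the character's capsule to the "Spawn" socket on the first BP_Spawner's Portal.
; It also sets the controller's rotation to match that socket.
; Walls flagged IsRoof skip the teleport.
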(event OnComponentHit(Box)
  (params (HitComponent :type Primitive%20Component%20Object%20Reference) (OtherActor :type Actor%20Object%20Reference) (OtherComp :type Primitive%20Component%20Object%20Reference) (NormalImpulse :type Vector :default "0, 0, 0") (Hit :type Hit%20Result%20Structure%20%28by%20ref%29))
  (if (not (Variables|Default|GetIsRoof))
    (bind _asbp_player_character (Utilities|Casting|CastToBP_PlayerCharacter OtherActor))
    (bind _outactors (Actor|GetAllActorsOfClass "/Game/Blueprints/Map/BP_Spawner.BP_Spawner_C"))
    (Transformation|SetWorldLocation (Variables|/Script/Engine.Character|GetCapsuleComponent _asbp_player_character) (Transformation|GetSocketLocation (Variables|/Game/Blueprints/Map/BP_Spawner.BP_Spawner_C|GetPortal (Utilities|Array|Get(acopy) _outactors)) "Spawn") false true)
    (Pawn|SetControlRotation (Pawn|GetController _asbp_player_character) (Transformation|GetSocketRotation (Variables|/Game/Blueprints/Map/BP_Spawner.BP_Spawner_C|GetPortal (Utilities|Array|Get(acopy) _outactors)) "Spawn"))))

(event EventBeginPlay)

(event Collision|EventActorBeginOverlap
  (params (OtherActor :type Actor%20Object%20Reference)))

(event EventTick
  (params (DeltaSeconds :type Float%20%28single-precision%29)))

(fn ConstructionScript)