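; BP_Tower_A4 is a Tier 4 tower Blueprint that turns its Aqua component toward the first entry in its Targets list.
; The RotateAquatoTarget event passes delta time to RotateAquaToTargetOverride, which does nothing when there are no targets.
; Otherwise it interpolates at constant speed toward the look-at rotation and applies only the yaw difference as a local rotation.
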(event EventBeginPlay
  (|CallParentFunction) ; This node is disabled and will not be called.\nDrag off pins to build functionality.
)

(event Collision|EventActorBeginOverlap
  (params (OtherActor :type Actor%20Object%20Reference))
  (|CallParentFunction OtherActor) ; This node is disabled and will not be called.\nDrag off pins to build functionality.
)

(event EventTick
  (params (DeltaSeconds :type Float%20%28single-precision%29))
  (|CallParentFunction DeltaSeconds) ; This node is disabled and will not be called.\nDrag off pins to build functionality.
)

(event EventRotateAquatoTarget
  (params (DeltaTime :type Float%20%28single-precision%29))
  (CallFunction|RotateAquatoTargetOverride DeltaTime))

(fn ConstructionScript
  (|CallParentFunction))

(fn RotateAquatoTargetOverride
  (params (DeltaTime :type Float%20%28single-precision%29))
  (bind _targets (Variables|Default|GetTargets))
  (bind _aqua (Variables|Default|GetAqua))
  (bind _returnvalue (Transformation|GetWorldTransform _aqua))
  (if (> (Utilities|Array|Length _targets) 0)
    (Transformation|AddLocalRotation _aqua (Math|Rotator|MakeRotator 0.0 0.0 (.yaw (Math|Rotator|CombineRotators (Class|KismetMathLibrary|RInterptoConstant (.rotation _returnvalue) (Math|Rotator|FindLookatRotation (.location _returnvalue) (Transformation|GetWorldLocation (Variables|/Script/Engine.Actor|GetRootComponent (Utilities|Array|Get(acopy) _targets)))) DeltaTime 2.5e+02) (Class|KismetMathLibrary|NegateRotator (.rotation _returnvalue))))) false false)))