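; BP_Tower_AA is a Tier A tower Blueprint that turns its WaterSword component toward the first entry in its Targets list.
; The RotateWaterSwordtoTarget event passes delta time to RotateWaterSwordToTargetOverride, which does nothing when there are no targets.
; Rotation uses constant-speed interpolation toward a look-at rotation, applying only the yaw difference as a local rotation.
; BeginPlay, overlap and Tick are disabled stubs.
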(event EventBeginPlay
  (|CallParentFunction) ; This node is disabled and will not be called.\nDrag off pins to build functionality.
)

(event Collision|EventActorBeginOverlap
  (params (OtherActor :type Actor%20Object%20Reference))
  (|CallParentFunction OtherActor) ; This node is disabled and will not be called.\nDrag off pins to build functionality.
)

(event EventTick
  (params (DeltaSeconds :type Float%20%28single-precision%29))
  (|CallParentFunction DeltaSeconds) ; This node is disabled and will not be called.\nDrag off pins to build functionality.
)

(event EventRotateWaterSwordtoTarget
  (params (Delta :type Float%20%28single-precision%29))
  (CallFunction|RotateWaterSwordtoTargetOverride Delta))

(fn ConstructionScript
  (|CallParentFunction))

(fn RotateWaterSwordtoTargetOverride
  (params (DeltaTime :type Float%20%28single-precision%29))
  (bind _targets (Variables|Default|GetTargets))
  (bind _watersword (Variables|Default|GetWaterSword))
  (bind _returnvalue (Transformation|GetWorldTransform _watersword))
  (if (> (Utilities|Array|Length _targets) 0)
    (Transformation|AddLocalRotation _watersword (Math|Rotator|MakeRotator 0.0 0.0 (.yaw (Math|Rotator|CombineRotators (Class|KismetMathLibrary|RInterptoConstant (.rotation _returnvalue) (Math|Rotator|FindLookatRotation (.location _returnvalue) (Transformation|GetWorldLocation (Variables|/Script/Engine.Actor|GetRootComponent (Utilities|Array|Get(acopy) _targets)))) DeltaTime 2.5e+02) (Class|KismetMathLibrary|NegateRotator (.rotation _returnvalue))))) false false)))