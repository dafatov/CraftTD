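; Tier 0 tower Blueprint with two clouds that serve as alternating bullet spawn points.
; On BeginPlay it starts a timeline per cloud, moving each one's relative X and Y while keeping its Z.
; The GetBulletSpawnTransform override toggles a flag each call to alternate between the clouds' "Bullet" sockets in world space, with the parent's transform as the fallback for a missing socket.
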(event Custom|Animation
  (|CloudsAnimation))

(event EventBeginPlay
  (|CallParentFunction)
  (CallFunction|Animation))

(event Collision|EventActorBeginOverlap
  (params (OtherActor :type Actor%20Object%20Reference)))

(event EventTick
  (params (DeltaSeconds :type Float%20%28single-precision%29)))

(fn ConstructionScript
  (|CallParentFunction))

(fn GetBulletSpawnTransform
  (if (Transformation|DoesSocketExist (select (Variables|Default|GetFlipFlop) (Variables|Default|GetCloud1) (Variables|Default|GetCloud0)) "Bullet")
    _
    (else
      (bind _returnvalue (|CallParentFunction))))
  (Variables|Default|SetFlipFlop (not (Variables|Default|GetFlipFlop)))
  (return (select (Transformation|DoesSocketExist (select (Variables|Default|GetFlipFlop) (Variables|Default|GetCloud1) (Variables|Default|GetCloud0)) "Bullet") (Transformation|GetSocketTransform (select (Variables|Default|GetFlipFlop) (Variables|Default|GetCloud1) (Variables|Default|GetCloud0)) "Bullet" "RTS_World") _returnvalue)))