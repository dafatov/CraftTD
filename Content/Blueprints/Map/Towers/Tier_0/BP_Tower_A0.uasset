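; BP_Tower_A0 is a Tier 0 map tower whose Aqua component swivels toward its current target.
; Each Tick rotates the status menu for players and turns Aqua at constant speed toward the first entry in Targets, following look-at yaw and roll but not pitch.
; It overrides GetBulletSpawnTransform to use Aqua's "Bullet" socket in world space, falling back to the parent's transform when that socket is missing.
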(event EventBeginPlay
  (|CallParentFunction) ; This node is disabled and will not be called.\nDrag off pins to build functionality.
)

(event Collision|EventActorBeginOverlap
  (params (OtherActor :type Actor%20Object%20Reference)))

(event EventTick
  (params (DeltaSeconds :type Float%20%28single-precision%29))
  (CallFunction|RotateStatusMenuforPlayers DeltaSeconds)
  (CallFunction|RotateAquatoTarget DeltaSeconds))

(fn ConstructionScript
  (|CallParentFunction))

(fn RotateAquatoTarget
  (params (DeltaTime :type Float%20%28single-precision%29))
  (bind _targets (Variables|Default|GetTargets))
  (bind _aqua (Variables|Default|GetAqua))
  (bind _returnvalue (Transformation|GetWorldTransform _aqua))
  (bind _output (Utilities|Array|Get(acopy) _targets))
  (bind _rootcomponent (Variables|/Script/Engine.Actor|GetRootComponent _output))
  (bind _returnvalue_2 (Transformation|GetWorldLocation _rootcomponent))
  (bind _returnvalue_3 (Math|Rotator|FindLookatRotation (.location _returnvalue) _returnvalue_2))
  (if (> (Utilities|Array|Length _targets) 0)
    (Transformation|SetWorldRotation _aqua (Class|KismetMathLibrary|RInterptoConstant (.rotation _returnvalue) (Math|Rotator|MakeRotator (.roll _returnvalue_3) 0.0 (.yaw _returnvalue_3)) DeltaTime 2.5e+02) false false)))

(fn GetBulletSpawnTransform
  (bind _aqua (Variables|Default|GetAqua))
  (bind _returnvalue (Transformation|DoesSocketExist _aqua "Bullet"))
  (if _returnvalue
    _
    (else
      (bind _returnvalue_2 (|CallParentFunction))))
  (return (select _returnvalue (Transformation|GetSocketTransform _aqua "Bullet" "RTS_World") _returnvalue_2)))