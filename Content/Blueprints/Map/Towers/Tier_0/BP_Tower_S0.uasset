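; BP_Tower_S0 is a Tier 0 tower Blueprint with a rotating Earth component.
; On BeginPlay it runs the parent logic, then plays the Rotation timeline to drive the Earth component's relative yaw.
; It overrides GetBulletSpawnTransform to return the world transform of Earth's Bullet socket, falling back to the parent implementation when that socket is missing.
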(event EventBeginPlay
  (|CallParentFunction)
  (bind _z (Timeline|Rotation PlayFromStart)
    (:Update
      (Transformation|SetRelativeRotation (Variables|Default|GetEarth) (Math|Rotator|MakeRotator 0.0 0.0 _z) false false))))

(event Collision|EventActorBeginOverlap
  (params (OtherActor :type Actor%20Object%20Reference)))

(fn ConstructionScript
  (|CallParentFunction))

(fn GetBulletSpawnTransform
  (bind _earth (Variables|Default|GetEarth))
  (bind _returnvalue (Transformation|DoesSocketExist _earth "Bullet"))
  (if _returnvalue
    _
    (else
      (bind _returnvalue_2 (|CallParentFunction))))
  (return (select _returnvalue (Transformation|GetSocketTransform _earth "Bullet" "RTS_World") _returnvalue_2)))