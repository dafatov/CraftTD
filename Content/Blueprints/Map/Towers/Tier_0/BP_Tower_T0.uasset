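; Tier 0 tower Blueprint that turns its BlackHole component toward a target and supplies the spawn transform for its bullets.
; Each tick it rotates the status menu for players and turns BlackHole at a constant interpolation speed to face the first entry in Targets.
; GetBulletSpawnTransform uses the BlackHole "Bullet" socket in world space, falling back to the parent implementation when that socket is missing.
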(event EventBeginPlay
  (|CallParentFunction) ; This node is disabled and will not be called.\nDrag off pins to build functionality.
)

(event Collision|EventActorBeginOverlap
  (params (OtherActor :type Actor%20Object%20Reference)))

(event EventTick
  (params (DeltaSeconds :type Float%20%28single-precision%29))
  (CallFunction|RotateStatusMenuforPlayers DeltaSeconds)
  (CallFunction|RotateBlackHoletoTarget DeltaSeconds))

(fn ConstructionScript
  (|CallParentFunction))

(fn RotateBlackHoletoTarget
  (params (DeltaTime :type Float%20%28single-precision%29))
  (bind _targets (Variables|Default|GetTargets))
  (bind _blackhole (Variables|Default|GetBlackHole))
  (bind _returnvalue (Transformation|GetWorldTransform _blackhole))
  (if (> (Utilities|Array|Length _targets) 0)
    (Transformation|SetWorldRotation _blackhole (Class|KismetMathLibrary|RInterptoConstant (.rotation _returnvalue) (Math|Rotator|FindLookatRotation (.location _returnvalue) (Transformation|GetWorldLocation (Variables|/Script/Engine.Actor|GetRootComponent (Utilities|Array|Get(acopy) _targets)))) DeltaTime 2.5e+02) false false)))

(fn GetBulletSpawnTransform
  (bind _blackhole (Variables|Default|GetBlackHole))
  (bind _returnvalue (Transformation|DoesSocketExist _blackhole "Bullet"))
  (if _returnvalue
    _
    (else
      (bind _returnvalue_2 (|CallParentFunction))))
  (return (select _returnvalue (Transformation|GetSocketTransform _blackhole "Bullet" "RTS_World") _returnvalue_2)))