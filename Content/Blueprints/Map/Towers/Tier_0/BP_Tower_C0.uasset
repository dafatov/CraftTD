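; BP_Tower_C0 is a Tier 0 tower whose Book component turns to face the first entry in its Targets list.
; Each tick it rotates the status menu for players and swings the book toward that target at a constant interpolation speed.
; It overrides the bullet spawn transform to use the book's "Bullet" socket, falling back to the parent's transform when that socket is missing.
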(event EventBeginPlay
  (|CallParentFunction) ; This node is disabled and will not be called.\nDrag off pins to build functionality.
)

(event Collision|EventActorBeginOverlap
  (params (OtherActor :type Actor%20Object%20Reference)))

(event EventTick
  (params (DeltaSeconds :type Float%20%28single-precision%29))
  (CallFunction|RotateStatusMenuforPlayers DeltaSeconds)
  (CallFunction|RotateBooktoTarget DeltaSeconds))

(fn ConstructionScript
  (|CallParentFunction))

(fn RotateBooktoTarget
  (params (DeltaTime :type Float%20%28single-precision%29))
  (bind _targets (Variables|Default|GetTargets))
  (bind _book (Variables|Default|GetBook))
  (bind _returnvalue (Transformation|GetWorldTransform _book))
  (if (> (Utilities|Array|Length _targets) 0)
    (Transformation|SetWorldRotation _book (Class|KismetMathLibrary|RInterptoConstant (.rotation _returnvalue) (Math|Rotator|FindLookatRotation (.location _returnvalue) (Transformation|GetWorldLocation (Variables|/Script/Engine.Actor|GetRootComponent (Utilities|Array|Get(acopy) _targets)))) DeltaTime 2.5e+02) false false)))

(fn GetBulletSpawnTransform
  (bind _book (Variables|Default|GetBook))
  (bind _returnvalue (Transformation|DoesSocketExist _book "Bullet"))
  (if _returnvalue
    _
    (else
      (bind _returnvalue_2 (|CallParentFunction))))
  (return (select _returnvalue (Transformation|GetSocketTransform _book "Bullet" "RTS_World") _returnvalue_2)))