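; BP_Tower_O0 is a Tier 0 map tower that turns to face its target and fires from two alternating muzzles.
; Each tick it updates the inherited status menu rotation and turns the Scales component at constant speed toward the first target, leaving pitch level.
; Its bullet spawn override alternates between two sockets on Scales via a flip-flop, falling back to the parent transform when the socket is missing.
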(event EventBeginPlay
  (|CallParentFunction) ; This node is disabled and will not be called.\nDrag off pins to build functionality.
)

(event Collision|EventActorBeginOverlap
  (params (OtherActor :type Actor%20Object%20Reference)))

(event EventTick
  (params (DeltaSeconds :type Float%20%28single-precision%29))
  (CallFunction|RotateStatusMenuforPlayers DeltaSeconds)
  (CallFunction|RotateScalestoTarget DeltaSeconds))

(fn ConstructionScript
  (|CallParentFunction))

(fn RotateScalestoTarget
  (params (DeltaTime :type Float%20%28single-precision%29))
  (bind _scales (Variables|Default|GetScales))
  (bind _targets (Variables|Default|GetTargets))
  (bind _returnvalue (Transformation|GetWorldTransform _scales))
  (bind _output (Utilities|Array|Get(acopy) _targets))
  (bind _rootcomponent (Variables|/Script/Engine.Actor|GetRootComponent _output))
  (bind _returnvalue_2 (Transformation|GetWorldLocation _rootcomponent))
  (bind _returnvalue_3 (Math|Rotator|FindLookatRotation (.location _returnvalue) _returnvalue_2))
  (if (> (Utilities|Array|Length _targets) 0)
    (Transformation|SetWorldRotation _scales (Class|KismetMathLibrary|RInterptoConstant (.rotation _returnvalue) (Math|Rotator|MakeRotator (.roll _returnvalue_3) 0.0 (.yaw _returnvalue_3)) DeltaTime 2.5e+02) false false)))

(fn GetBulletSpawnTransform
  (bind _scales (Variables|Default|GetScales))
  (if (Transformation|DoesSocketExist _scales (Utilities|Name|MakeLiteralName (select (Variables|Default|GetFlipFlop) "Bullet2" "Bullet")))
    _
    (else
      (bind _returnvalue (|CallParentFunction))))
  (Variables|Default|SetFlipFlop (not (Variables|Default|GetFlipFlop)))
  (return (select (Transformation|DoesSocketExist _scales (Utilities|Name|MakeLiteralName (select (Variables|Default|GetFlipFlop) "Bullet2" "Bullet"))) (Transformation|GetSocketTransform _scales (Utilities|Name|MakeLiteralName (select (Variables|Default|GetFlipFlop) "Bullet2" "Bullet")) "RTS_World") _returnvalue)))