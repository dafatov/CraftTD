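; BP_Tower_P0 is a Tier 0 tower Blueprint that plays an earth destructible effect above itself and supplies a bullet spawn transform.
; On BeginPlay, the Animation timeline's event tracks add a scaled-down destructible component, shatter it with damage, then destroy it.
; A shared helper returns a fixed vertical offset, placing the earth component and, added to the Tower's world location, the bullet spawn point.
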(event EventBeginPlay
  (|CallParentFunction)
  (Timeline|Animation PlayFromStart
    (:Create
      (bind _returnvalue (CallFunction|GetRelativeSpawnLocationEarthDM))
      (bind _returnvalue_2 (AddComponent|AddDestructibleComponent false (Math|Transform|MakeTransform _returnvalue "0, 0, 0" "0.700000,0.700000,0.700000")))
      (bind _output_get (Variables|Default|SetEarth _returnvalue_2)))
    (:Explode
      (Class|DestructibleComponent|ApplyDamage _output_get 1e+02 (Transformation|GetWorldLocation _output_get) (Math|Vector|MakeVector 0.0 0.0 0.0) 1e+01))
    (:Destroy
      (Components|DestroyComponent _output_get))))

(fn ConstructionScript
  (|CallParentFunction))

(fn GetBulletSpawnTransform
  (bind _returnvalue (CallFunction|GetRelativeSpawnLocationEarthDM))
  (return (Math|Conversions|ToTransform(Vector) (+ _returnvalue (Transformation|GetWorldLocation (Variables|Default|GetTower))))))

(fn GetRelativeSpawnLocationEarthDM
  (return (Math|Vector|MakeVector 0.0 0.0 3e+02)))