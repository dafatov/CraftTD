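; BP_Tower_CD is a Tier D tower Blueprint with a scythe that tracks its first target and serves as the bullet origin.
; Each tick rotates the scythe toward the target at constant speed, adding a timeline-driven roll offset.
; The swept rotation lets scythe hits on the tower mesh trigger brief, non-overlapping spark bursts.
; Bullet spawns alternate between two scythe sockets, with the parent transform as fallback.
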(event OnComponentHit(Scythe2)
  (params (HitComponent :type Primitive%20Component%20Object%20Reference) (OtherActor :type Actor%20Object%20Reference) (OtherComp :type Primitive%20Component%20Object%20Reference) (NormalImpulse :type Vector :default "0, 0, 0") (Hit :type Hit%20Result%20Structure%20%28by%20ref%29)))

(event OnComponentHit(Scythe)
  (params (HitComponent :type Primitive%20Component%20Object%20Reference) (OtherActor :type Actor%20Object%20Reference) (OtherComp :type Primitive%20Component%20Object%20Reference) (NormalImpulse :type Vector :default "0, 0, 0") (Hit :type Hit%20Result%20Structure%20%28by%20ref%29))
  (bind _asstatic_mesh_component (Utilities|Casting|CastToStaticMeshComponent OtherComp))
  (if (== _asstatic_mesh_component (Variables|Default|GetTower))
    (CallFunction|Animation (.location Hit))))

(event Custom|Animation
  (params (Location :type Vector))
  (bind _sparks (Variables|Default|GetSparks)
    (:then)
    (:else
      (bind _returnvalue (Effects|SpawnEmitteratLocation "/Game/StarterContent/Particles/P_Sparks.P_Sparks" Location "0, 0, 0" "1.000000,1.000000,1.000000" false))
      (Variables|Default|SetSparks _returnvalue)
      (Utilities|FlowControl|Delay 0.1)
      (Components|DestroyComponent _sparks))))

(event EventBeginPlay
  (|CallParentFunction)
  (bind _rotation (Timeline|Animate PlayFromStart)
    (:Update
      (Variables|Default|SetFloatOffset _rotation))))

(event Collision|EventActorBeginOverlap
  (params (OtherActor :type Actor%20Object%20Reference)))

(event EventTick
  (params (DeltaSeconds :type Float%20%28single-precision%29))
  (|CallParentFunction DeltaSeconds)
  (CallFunction|RotateScythetoTarget DeltaSeconds))

(fn ConstructionScript
  (|CallParentFunction))

(fn GetBulletSpawnTransform
  (bind _scythe (Variables|Default|GetScythe))
  (if (Transformation|DoesSocketExist _scythe (Utilities|Name|MakeLiteralName (select (Variables|Default|GetFlipFlop) "Bullet2" "Bullet")))
    _
    (else
      (bind _returnvalue (|CallParentFunction))))
  (Variables|Default|SetFlipFlop (not (Variables|Default|GetFlipFlop)))
  (return (select (Transformation|DoesSocketExist _scythe (Utilities|Name|MakeLiteralName (select (Variables|Default|GetFlipFlop) "Bullet2" "Bullet"))) (Transformation|GetSocketTransform _scythe (Utilities|Name|MakeLiteralName (select (Variables|Default|GetFlipFlop) "Bullet2" "Bullet")) "RTS_World") _returnvalue)))

(fn RotateScythetoTarget
  (params (Delta :type Float%20%28single-precision%29))
  (bind _targets (Variables|Default|GetTargets))
  (bind _scythe (Variables|Default|GetScythe))
  (bind _returnvalue (Transformation|GetWorldTransform _scythe))
  (bind _output (Utilities|Array|Get(acopy) _targets))
  (bind _rootcomponent (Variables|/Script/Engine.Actor|GetRootComponent _output))
  (bind _returnvalue_2 (Transformation|GetWorldLocation _rootcomponent))
  (bind _returnvalue_3 (Math|Rotator|FindLookatRotation (.location _returnvalue) _returnvalue_2))
  (bind (_roll _pitch _yaw) (Math|Rotator|BreakRotator _returnvalue_3))
  (if (> (Utilities|Array|Length _targets) 0)
    (Transformation|SetWorldRotation _scythe (Class|KismetMathLibrary|RInterptoConstant (.rotation _returnvalue) (Math|Rotator|MakeRotator (+ _roll (Variables|Default|GetFloatOffset)) _pitch _yaw) Delta 2.5e+02) true false)))