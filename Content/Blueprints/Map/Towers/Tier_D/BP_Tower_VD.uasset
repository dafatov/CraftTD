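; Tier D tower Blueprint that aims two Kirito sword components and alternates bullet spawns between them, extending a parent tower.
; Each tick, both swords turn toward the first entry in Targets at a constant interpolated rate, with pitch clamped to a different upper limit per sword.
; The GetBulletSpawnTransform override toggles a FlipFlop boolean to pick a sword's Bullet socket, falling back to the parent transform when the socket is missing.
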(event EventBeginPlay
  (|CallParentFunction) ; This node is disabled and will not be called.\nDrag off pins to build functionality.
)

(event Collision|EventActorBeginOverlap
  (params (OtherActor :type Actor%20Object%20Reference)))

(event EventTick
  (params (DeltaSeconds :type Float%20%28single-precision%29))
  (|CallParentFunction DeltaSeconds)
  (CallFunction|RotateSword1toTarget DeltaSeconds)
  (CallFunction|RotateSword2toTarget DeltaSeconds))

(fn ConstructionScript
  (|CallParentFunction))

(fn GetBulletSpawnTransform
  (if (Transformation|DoesSocketExist (select (Variables|Default|GetFlipFlop) (Variables|Default|GetKiritoSword2) (Variables|Default|GetKiritoSword1)) "Bullet")
    _
    (else
      (bind _returnvalue (|CallParentFunction))))
  (Variables|Default|SetFlipFlop (not (Variables|Default|GetFlipFlop)))
  (return (select (Transformation|DoesSocketExist (select (Variables|Default|GetFlipFlop) (Variables|Default|GetKiritoSword2) (Variables|Default|GetKiritoSword1)) "Bullet") (Transformation|GetSocketTransform (select (Variables|Default|GetFlipFlop) (Variables|Default|GetKiritoSword2) (Variables|Default|GetKiritoSword1)) "Bullet" "RTS_World") _returnvalue)))

(fn RotateSword1toTarget
  (params (Delta :type Float%20%28single-precision%29))
  (bind _targets (Variables|Default|GetTargets))
  (bind _kiritosword1 (Variables|Default|GetKiritoSword1))
  (bind _returnvalue (Transformation|GetWorldTransform _kiritosword1))
  (bind _output (Utilities|Array|Get(acopy) _targets))
  (bind _rootcomponent (Variables|/Script/Engine.Actor|GetRootComponent _output))
  (bind _returnvalue_2 (Transformation|GetWorldLocation _rootcomponent))
  (bind _returnvalue_3 (Math|Rotator|FindLookatRotation (.location _returnvalue) _returnvalue_2))
  (bind _returnvalue_4 (Class|KismetMathLibrary|RInterptoConstant (.rotation _returnvalue) _returnvalue_3 Delta 2.5e+02))
  (if (> (Utilities|Array|Length _targets) 0)
    (Transformation|SetWorldRotation _kiritosword1 (Math|Rotator|MakeRotator (.roll _returnvalue_4) (Math|Float|Clamp(Float) (.pitch _returnvalue_4) -2e+01 9e+01) (.yaw _returnvalue_4)) false false)))

(fn RotateSword2toTarget
  (params (Delta :type Float%20%28single-precision%29))
  (bind _kiritosword2 (Variables|Default|GetKiritoSword2))
  (bind _targets (Variables|Default|GetTargets))
  (bind _returnvalue (Transformation|GetWorldTransform _kiritosword2))
  (bind _output (Utilities|Array|Get(acopy) _targets))
  (bind _rootcomponent (Variables|/Script/Engine.Actor|GetRootComponent _output))
  (bind _returnvalue_2 (Transformation|GetWorldLocation _rootcomponent))
  (bind _returnvalue_3 (Math|Rotator|FindLookatRotation (.location _returnvalue) _returnvalue_2))
  (bind _returnvalue_4 (Class|KismetMathLibrary|RInterptoConstant (.rotation _returnvalue) _returnvalue_3 Delta 2.5e+02))
  (if (> (Utilities|Array|Length _targets) 0)
    (Transformation|SetWorldRotation _kiritosword2 (Math|Rotator|MakeRotator (.roll _returnvalue_4) (Math|Float|Clamp(Float) (.pitch _returnvalue_4) -2e+01 35.0) (.yaw _returnvalue_4)) false false)))