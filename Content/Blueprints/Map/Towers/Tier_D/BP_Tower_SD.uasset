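; BP_Tower_SD is a tower Blueprint, filed under Tier D, whose ZoroSword component aims at the first entry in its Targets list.
; Each tick, after the parent logic, the sword turns toward that target at a constant rate, with pitch clamped to a limited range.
; It overrides the bullet spawn transform to use the sword's "Bullet" socket, falling back to the parent's transform when that socket is missing.
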(event EventBeginPlay
  (|CallParentFunction) ; This node is disabled and will not be called.\nDrag off pins to build functionality.
)

(event Collision|EventActorBeginOverlap
  (params (OtherActor :type Actor%20Object%20Reference)))

(event EventTick
  (params (DeltaSeconds :type Float%20%28single-precision%29))
  (|CallParentFunction DeltaSeconds)
  (CallFunction|RotateSwordtoTarget DeltaSeconds))

(fn ConstructionScript
  (|CallParentFunction))

(fn RotateSwordtoTarget
  (params (Delta :type Float%20%28single-precision%29))
  (bind _zorosword (Variables|Default|GetZoroSword))
  (bind _targets (Variables|Default|GetTargets))
  (bind _returnvalue (Transformation|GetWorldTransform _zorosword))
  (bind _output (Utilities|Array|Get(acopy) _targets))
  (bind _rootcomponent (Variables|/Script/Engine.Actor|GetRootComponent _output))
  (bind _returnvalue_2 (Transformation|GetWorldLocation _rootcomponent))
  (bind _returnvalue_3 (Math|Rotator|FindLookatRotation (.location _returnvalue) _returnvalue_2))
  (bind _returnvalue_4 (Class|KismetMathLibrary|RInterptoConstant (.rotation _returnvalue) _returnvalue_3 Delta 2.5e+02))
  (if (> (Utilities|Array|Length _targets) 0)
    (Transformation|SetWorldRotation _zorosword (Math|Rotator|MakeRotator (.roll _returnvalue_4) (Math|Float|Clamp(Float) (.pitch _returnvalue_4) -35.0 25.0) (.yaw _returnvalue_4)) false false)))

(fn GetBulletSpawnTransform
  (bind _zorosword (Variables|Default|GetZoroSword))
  (bind _returnvalue (Transformation|DoesSocketExist _zorosword "Bullet"))
  (if _returnvalue
    _
    (else
      (bind _returnvalue_2 (|CallParentFunction))))
  (return (select _returnvalue (Transformation|GetSocketTransform _zorosword "Bullet" "RTS_World") _returnvalue_2)))