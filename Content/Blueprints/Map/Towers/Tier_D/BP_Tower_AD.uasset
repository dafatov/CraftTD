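; BP_Tower_AD is a Tier D tower that aims a WaterSword component at its targets and uses it as the bullet spawn point.
; Each Tick, it turns the sword toward the first entry in Targets at a constant interpolation speed.
; GetBulletSpawnTransform returns the sword's Bullet socket in world space, falling back to the parent's transform when that socket is missing.
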(event EventBeginPlay
  (|CallParentFunction) ; This node is disabled and will not be called.\nDrag off pins to build functionality.
)

(event Collision|EventActorBeginOverlap
  (params (OtherActor :type Actor%20Object%20Reference)))

(event EventTick
  (params (DeltaSeconds :type Float%20%28single-precision%29))
  (|CallParentFunction DeltaSeconds)
  (CallFunction|RotateWaterSwordtoTarget DeltaSeconds))

(fn ConstructionScript
  (|CallParentFunction))

(fn GetBulletSpawnTransform
  (bind _watersword (Variables|Default|GetWaterSword))
  (bind _returnvalue (Transformation|DoesSocketExist _watersword "Bullet"))
  (if _returnvalue
    _
    (else
      (bind _returnvalue_2 (|CallParentFunction))))
  (return (select _returnvalue (Transformation|GetSocketTransform _watersword "Bullet" "RTS_World") _returnvalue_2)))

(fn RotateWaterSwordtoTarget
  (params (Delta :type Float%20%28single-precision%29))
  (bind _watersword (Variables|Default|GetWaterSword))
  (bind _targets (Variables|Default|GetTargets))
  (bind _returnvalue (Transformation|GetWorldTransform _watersword))
  (if (> (Utilities|Array|Length _targets) 0)
    (Transformation|SetWorldRotation _watersword (Class|KismetMathLibrary|RInterptoConstant (.rotation _returnvalue) (Math|Rotator|FindLookatRotation (.location _returnvalue) (Transformation|GetWorldLocation (Variables|/Script/Engine.Actor|GetRootComponent (Utilities|Array|Get(acopy) _targets)))) Delta 2.5e+02) false false)))