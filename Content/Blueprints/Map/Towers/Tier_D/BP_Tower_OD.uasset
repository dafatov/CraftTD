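; BP_Tower_OD is a Tier D tower with a sword as its aiming turret, firing from the sword's Bullet socket when present.
; Each tick it rotates the sword at constant speed toward the first target, with pitch clamped.
; Paired DoOnce nodes toggle the scabbard (Cabbard): it is flung off with physics when targets appear and snaps back onto the sword when none remain.
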(event EventBeginPlay
  (|CallParentFunction) ; This node is disabled and will not be called.\nDrag off pins to build functionality.
)

(event Collision|EventActorBeginOverlap
  (params (OtherActor :type Actor%20Object%20Reference)))

(event EventTick
  (params (DeltaSeconds :type Float%20%28single-precision%29))
  (|CallParentFunction DeltaSeconds)
  (CallFunction|RotateSwordtoTarget DeltaSeconds))

(fn ConstructionScript
  (|CallParentFunction))

(fn GetBulletSpawnTransform
  (bind _sword (Variables|Default|GetSword))
  (bind _returnvalue (Transformation|DoesSocketExist _sword "Bullet"))
  (if _returnvalue
    _
    (else
      (bind _returnvalue_2 (|CallParentFunction))))
  (return (select _returnvalue (Transformation|GetSocketTransform _sword "Bullet" "RTS_World") _returnvalue_2)))

(fn RotateSwordtoTarget
  (params (Delta :type Float%20%28single-precision%29))
  (bind _sword (Variables|Default|GetSword))
  (bind _targets (Variables|Default|GetTargets))
  (bind _cabbard (Variables|Default|GetCabbard))
  (bind _cabbard_2 (Variables|Default|GetCabbard))
  (bind _returnvalue (Transformation|GetWorldTransform _sword))
  (bind _output (Utilities|Array|Get(acopy) _targets))
  (bind _rootcomponent (Variables|/Script/Engine.Actor|GetRootComponent _output))
  (bind _returnvalue_2 (Transformation|GetWorldLocation _rootcomponent))
  (bind _returnvalue_3 (Math|Rotator|FindLookatRotation (.location _returnvalue) _returnvalue_2))
  (bind _returnvalue_4 (Class|KismetMathLibrary|RInterptoConstant (.rotation _returnvalue) _returnvalue_3 Delta 2.5e+02))
  (if (> (Utilities|Array|Length _targets) 0)
    (Transformation|SetWorldRotation _sword (Math|Rotator|MakeRotator (.roll _returnvalue_4) (Math|Float|Clamp(Float) (.pitch _returnvalue_4) -3e+01 9e+01) (.yaw _returnvalue_4)) false false)
    (Utilities|FlowControl|Sequence
      (:then_0
        (goto _label_2 Reset))
      (:then_1
        (Utilities|FlowControl|DoOnce false :!label _label
          (:Completed
            (Physics|SetSimulatePhysics _cabbard_2 true)
            (Physics|AddForce _cabbard_2 (* (Math|Vector|GetForwardVector _cabbard_2) 2e+03) "None" false)))))
    (else
      (Utilities|FlowControl|Sequence
        (:then_0
          (goto _label Reset))
        (:then_1
          (Utilities|FlowControl|DoOnce false :!label _label_2
            (:Completed
              (Physics|SetSimulatePhysics _cabbard false)
              (Transformation|SetWorldTransform _cabbard (Transformation|GetWorldTransform (Variables|Default|GetSword)) false false))))))))