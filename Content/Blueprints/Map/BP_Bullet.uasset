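; Homing tower projectile that chases a mob, retargeting to the Damager's first target if auto-targeting, else destroying itself.
; BeginPlay sets its look by animation type: borrowed tower mesh, material sphere, or particles attached to the bullet or emitted from a source socket toward the target.
; On overlapping its target, the server applies damage plus optional slow, explosion, rewind, lone-target bonus and bounce effects.
; Bounces respawn bullets through the Damager with scaled damage and a decremented counter.
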(event OnComponentBeginOverlap(StaticMeshObject)
  (params (OverlappedComponent :type Primitive%20Component%20Object%20Reference) (OtherActor :type Actor%20Object%20Reference) (OtherComp :type Primitive%20Component%20Object%20Reference) (OtherBodyIndex :type Integer) (bFromSweep :type Boolean) (SweepResult :type Hit%20Result%20Structure%20%28by%20ref%29))
  (bind _target (Variables|Default|GetTarget))
  ;[1 1 1] Damage target when overlaps
  (if (== OtherActor _target)
    (if (Networking|IsServer)
      (bind _returnvalue (Game|Damage|ApplyDamage _target (Variables|Default|GetDamage) 0 (Variables|Default|GetDamager)))
      (Variables|Default|SetTotalDamage (+ _returnvalue (Variables|Default|GetTotalDamage)))
      (if (Variables|Attributes|GetHasSlowEffect?)
        (Default|SlowMovement _target (Variables|Attributes|GetSlowAlpha) (Variables|Attributes|GetSlowTime)))
      (if (Variables|Attributes|GetHasExplosionEffect?)
        (CallFunction|DoExplosionDamage (Variables|Attributes|GetExplosionRadius) (Variables|Attributes|GetExplosionAlpha) _target))
      (if (Variables|Attributes|GetHasBackTimeEffect?)
        (Default|BackLocationtoPast _target (Variables|Attributes|GetBackTime)))
      (if (Variables|Attributes|GetHasBouncingEffect?)
        (CallFunction|DoBouncingDamage _target (Variables|Attributes|GetBouncingRadius) (Variables|Attributes|GetBouncingAlpha) (Variables|Attributes|GetBouncingCounter)))
      (if (Variables|Attributes|GetHasExtraDmgLone?)
        (CallFunction|DoExtraDmgLone (Variables|Default|GetTarget) (Variables|Attributes|GetExtraDmgLoneRadius) (Variables|Attributes|GetExtraDmgLoneAlpha)))
      (Default|DamageApplied (Variables|Default|GetDamager) (Variables|Default|GetTotalDamage)))
    (Actor|DestroyActor)))

(event EventBeginPlay
  (bind _bulletanimationtype (Variables|Attributes|GetBulletAnimationType))
  (bind _asgi_info (Utilities|Casting|CastToGI_Info (Game|GetGameInstance)))
  (Variables|Default|SetGameInstanceRef _asgi_info)
  (switch Utilities|FlowControl|Switch|SwitchonE_BulletAnimationType _bulletanimationtype
    (:NewEnumerator0
      (|StaticMeshAnimation))
    (:NewEnumerator1
      (|CustomMaterialSphere _bulletanimationtype :!label _label))
    (:NewEnumerator5
      (goto _label))
    (:NewEnumerator9
      (goto _label))
    (:NewEnumerator10
      (goto _label))
    (:NewEnumerator2
      (|ParticleSystemAnimation(AttachedBullet) _bulletanimationtype :!label _label_2))
    (:NewEnumerator6
      (goto _label_2))
    (:NewEnumerator7
      (goto _label_2))
    (:NewEnumerator3
      (|ParticleSystemAnimation(AtachedTower) _bulletanimationtype :!label _label_3))
    (:NewEnumerator4
      (goto _label_3))))

(event EventDestroyed
  (bind _particlesystem (Variables|Default|GetParticleSystem)
    (:then
      (Components|DestroyComponent _particlesystem))
    (:else)))

(event EventTick
  (params (DeltaSeconds :type Float%20%28single-precision%29))
  (bind _damager (Variables|Default|GetDamager))
  (bind _defaultsceneroot (Variables|Default|GetDefaultSceneRoot))
  (bind _returnvalue (Transformation|GetWorldLocation _defaultsceneroot))
  (bind _targets (Variables|/Game/Blueprints/Map/BP_Tower.BP_Tower_C|GetTargets _damager))
  ;[1 1 1] Every Tick move to target
  (Networking|SwitchHasAuthority
    (:Authority
      _)
    (:Remote
      _))
  (Utilities|IsValid (Variables|Default|GetTarget)
    (:Is%20Valid
      (if (Variables|/Game/Blueprints/AI/Mobs/AI_Mob.AI_Mob_C|GetisDead (Variables|Default|GetTarget))
        (Default|TargetDeath (Variables|Default|GetDamager) (Variables|Default|GetTarget))
        (if (Math|Boolean|NANDBoolean (!= (Utilities|Array|Length _targets) 0) (Variables|Attributes|GetIsAutoTarget)) :!label _label
          (Actor|DestroyActor)
          (else
            (Variables|Default|SetTarget (Utilities|Array|Get(acopy) _targets))))
        (else
          (Transformation|SetWorldLocationAndRotation (Variables|Default|GetDefaultSceneRoot) (Math|Interpolation|VInterptoConstant _returnvalue (Transformation|GetWorldLocation (Variables|/Script/Engine.Actor|GetRootComponent (Variables|Default|GetTarget))) DeltaSeconds (* (Variables|/Game/Blueprints/Map/BP_Tower.BP_Tower_C|GetBulletSpeed _damager) (Variables|Default|GetSpeedAlphaAnimation))) (Math|Rotator|FindLookatRotation _returnvalue (Transformation|GetWorldLocation (Variables|/Script/Engine.Actor|GetRootComponent (Variables|Default|GetTarget)))) false false))))
    (:Is%20Not%20Valid
      (goto _label))))

(fn ConstructionScript)

(fn DoExplosionDamage
  (params (ExplosionRadius :type Integer) (ExplosionAlpha :type Float%20%28single-precision%29) (Target :type AI%20Mob%20Object%20Reference))
  (bind _alreadydamagedactors (LocalVariables|GetAlreadyDamagedActors))
  (bind _hitresults (CallFunction|MultiSphereTracePawns Target (Transformation|GetActorLocation) ExplosionRadius))
  (for _array_element _hitresults
    (if (and (== "/Game/Blueprints/AI/Mobs/AI_Mob.AI_Mob_C" (Utilities|GetClass (.HitActor (Collision|BreakHitResult _array_element)))) (not (Utilities|Set|Contains _alreadydamagedactors (.HitActor (Collision|BreakHitResult _array_element)))))
      (bind _returnvalue (Game|Damage|ApplyDamage (.HitActor (Collision|BreakHitResult _array_element)) (* ExplosionAlpha (Variables|Default|GetDamage)) 0 (Variables|Default|GetDamager)))
      (Variables|Default|SetTotalDamage (+ _returnvalue (Variables|Default|GetTotalDamage)))
      (Utilities|Set|Add _alreadydamagedactors (.HitActor (Collision|BreakHitResult _array_element))))))

(fn MultiSphereTracePawns
  (params (Target :type Actor%20Object%20Reference) (Center :type Vector) (Radius :type Integer))
  (bind _outhits (Collision|MultiSphereTraceForObjects Center (+ Center 0.1) (Math|Conversions|ToFloat(Integer) (+ (* Radius 200) 100)) (Utilities|Array|MakeArray "ObjectTypeQuery3") false (Utilities|Array|MakeArray Target) "None" true "(R=1.000000,G=0.000000,B=0.000000,A=1.000000)" "(R=0.000000,G=1.000000,B=0.000000,A=1.000000)" 3.0))
  (return _outhits))

(fn DoBouncingDamage
  (params (Target :type Actor%20Object%20Reference) (BouncingRadius :type Integer) (BouncingAlpha :type Float%20%28single-precision%29) (BouncingCounter :type Integer))
  (bind _returnvalue (Transformation|GetActorLocation))
  (bind _damager (Variables|Default|GetDamager))
  (bind _alreadycheckedactors (LocalVariables|GetAlreadyCheckedActors))
  (LocalVariables|SetClosestDistance 9.223372036854776e+18)
  (bind _hitresults (CallFunction|MultiSphereTracePawns Target _returnvalue BouncingRadius))
  (for _array_element _hitresults
    (if (and (== "/Game/Blueprints/AI/Mobs/AI_Mob.AI_Mob_C" (Utilities|GetClass (.HitActor (Collision|BreakHitResult _array_element)))) (not (Utilities|Set|Contains _alreadycheckedactors (.HitActor (Collision|BreakHitResult _array_element)))))
      (Utilities|Set|Add _alreadycheckedactors (.HitActor (Collision|BreakHitResult _array_element)))
      (if (< (Math|Vector|Distance(Vector) _returnvalue (Transformation|GetActorLocation (.HitActor (Collision|BreakHitResult _array_element)))) (LocalVariables|GetClosestDistance))
        (LocalVariables|SetClosestDistance (Math|Vector|Distance(Vector) _returnvalue (Transformation|GetActorLocation (.HitActor (Collision|BreakHitResult _array_element)))))
        (LocalVariables|SetClosestActor (.HitActor (Collision|BreakHitResult _array_element))))))
  (if (> BouncingCounter 0)
    (bind _asai_mob (Utilities|Casting|CastToAI_Mob (LocalVariables|GetClosestActor)))
    (Default|SpawnBullet-All _damager (Transformation|GetActorTransform) _asai_mob _damager (Variables|Attributes|GetBulletAnimationType) (Variables|Attributes|GetIsAutoTarget) (Variables|Attributes|GetSlowAlpha) (Variables|Attributes|GetSlowTime) (Variables|Attributes|GetHasSlowEffect?) (Variables|Attributes|GetHasExplosionEffect?) (Variables|Attributes|GetExplosionRadius) (Variables|Attributes|GetExplosionAlpha) (Variables|Attributes|GetHasBackTimeEffect?) (Variables|Attributes|GetBackTime) (Variables|Attributes|GetHasBouncingEffect?) (Variables|Attributes|GetBouncingRadius) (Variables|Attributes|GetBouncingAlpha) (- (Variables|Attributes|GetBouncingCounter) 1) (* (Variables|Default|GetDamage) BouncingAlpha) (Variables|Attributes|GetHasExtraDmgLone?) (Variables|Attributes|GetExtraDmgLoneRadius) (Variables|Attributes|GetExtraDmgLoneAlpha) true (Variables|/Script/Engine.Character|GetMesh (Variables|Default|GetTarget)))))

(fn DoExtraDmgLone
  (params (Target :type AI%20Mob%20Object%20Reference) (ExtraDmgLoneRadius :type Integer) (ExtraDmgLoneAlpha :type Float%20%28single-precision%29))
  (LocalVariables|SetHasMobsInRange false)
  (bind _hitresults (CallFunction|MultiSphereTracePawns Target (Transformation|GetActorLocation) ExtraDmgLoneRadius))
  (bind _array_element (Utilities|Array|ForEachLoopwithBreak _hitresults :!label _label)
    (:LoopBody
      (Utilities|Casting|CastToAI_Mob (.HitActor (Collision|BreakHitResult _array_element)))
      (LocalVariables|SetHasMobsInRange true)
      (goto _label Break))
    (:Completed
      (if (not (LocalVariables|GetHasMobsInRange))
        (bind _returnvalue (Game|Damage|ApplyDamage Target (* (Variables|Default|GetDamage) ExtraDmgLoneAlpha) 0 self))
        (Variables|Default|SetTotalDamage (+ _returnvalue (Variables|Default|GetTotalDamage)))))))