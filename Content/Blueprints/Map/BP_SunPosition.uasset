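; Map sun controller that keeps the sun in step with real-world UTC date and time.
; On BeginPlay and every minute by looping timers, it copies the current UTC time into its date and time variables and calls UpdateSun.
; It also reads SunHeight from BP_Sky_Sphere and, when night state changes, switches SpotLights with components tagged SpotLightGameboard on at night and off by day.
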(event Custom|SetMaterialByTime
  (bind _outactors (Actor|GetAllActorsOfClass "/Engine/EngineSky/BP_Sky_Sphere.BP_Sky_Sphere_C"))
  (if (not (Math|Boolean|Equal(Boolean) (< (Variables|/Engine/EngineSky/BP_Sky_Sphere.BP_Sky_Sphere_C|GetSun%20height (Utilities|Array|Get(acopy) _outactors)) 0.0) (Variables|Default|GetIsNight)))
    (bind _output_get (Variables|Default|SetIsNight (< (Variables|/Engine/EngineSky/BP_Sky_Sphere.BP_Sky_Sphere_C|GetSun%20height (Utilities|Array|Get(acopy) _outactors)) 0.0)))
    (bind _outactors_2 (Actor|GetAllActorsOfClass "/Script/Engine.SpotLight"))
    (bind _array_element (Utilities|Array|ForEachLoopwithBreak _outactors_2)
      (:LoopBody
        (if (Components|ComponentHasTag (Variables|/Script/Engine.Light|GetLightComponent _array_element) "SpotLightGameboard")
          (Rendering|Components|Light|SetIntensity (Variables|/Script/Engine.Light|GetLightComponent _array_element) (Math|Float|SelectFloat 5e+06 0.0 _output_get)))))))

(event Custom|UpdateTimeTimer
  (bind _returnvalue (Math|DateTime|UTCNow))
  (bind (_year _month _day _hour _minute _second) (Math|DateTime|BreakDateTime _returnvalue))
  (Variables|Default|SetYear _year)
  (Variables|Default|SetMonth _month)
  (Variables|Default|SetDay _day)
  (Variables|Default|SetHours _hour)
  (Variables|Default|SetMinutes _minute)
  (Variables|Default|SetSeconds _second)
  (CallFunction|UpdateSun))

(event EventBeginPlay
  (bind _returnvalue (Math|DateTime|UTCNow))
  (bind (_year _month _day _hour _minute _second) (Math|DateTime|BreakDateTime _returnvalue))
  (Utilities|FlowControl|Sequence
    (:then_0
      (Variables|Default|SetYear _year)
      (Variables|Default|SetMonth _month)
      (Variables|Default|SetDay _day)
      (Variables|Default|SetHours _hour)
      (Variables|Default|SetMinutes _minute)
      (Variables|Default|SetSeconds _second)
      (CallFunction|UpdateSun))
    (:then_1
      (bind _outactors (Actor|GetAllActorsOfClass "/Engine/EngineSky/BP_Sky_Sphere.BP_Sky_Sphere_C"))
      (if (not (Math|Boolean|Equal(Boolean) (< (Variables|/Engine/EngineSky/BP_Sky_Sphere.BP_Sky_Sphere_C|GetSun%20height (Utilities|Array|Get(acopy) _outactors)) 0.0) (Variables|Default|GetIsNight)))
        (bind _output_get (Variables|Default|SetIsNight (< (Variables|/Engine/EngineSky/BP_Sky_Sphere.BP_Sky_Sphere_C|GetSun%20height (Utilities|Array|Get(acopy) _outactors)) 0.0)))
        (bind _outactors_2 (Actor|GetAllActorsOfClass "/Script/Engine.SpotLight"))
        (bind _array_element (Utilities|Array|ForEachLoopwithBreak _outactors_2)
          (:LoopBody
            (if (Components|ComponentHasTag (Variables|/Script/Engine.Light|GetLightComponent _array_element) "SpotLightGameboard")
              (Rendering|Components|Light|SetIntensity (Variables|/Script/Engine.Light|GetLightComponent _array_element) (Math|Float|SelectFloat 5e+06 0.0 _output_get)))))))
    (:then_2
      (Utilities|Time|SetTimerbyEvent (delegate Custom|UpdateTimeTimer) 6e+01 true)
      (Utilities|Time|SetTimerbyEvent (delegate Custom|SetMaterialByTime) 6e+01 true))))

(fn ConstructionScript
  (|CallParentFunction))