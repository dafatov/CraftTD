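; Tower-defense tower that fires BP_Bullets with configurable effects at AI_Mobs inside its radius, optionally several at once.
; The authority tracks overlaps and runs a looping shot timer, spawning bullets through an "All" event.
; Optional effects bank bonus damage while idle or speed up itself and nearby towers by scaling fire delay.
; It also keeps a sorted damage-share ranking in GI_Info and rotates its status widget toward the player.
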(event OnComponentBeginOverlap(TowerDamager)
  (params (OverlappedComponent :type Primitive%20Component%20Object%20Reference) (OtherActor :type Actor%20Object%20Reference) (OtherComp :type Primitive%20Component%20Object%20Reference) (OtherBodyIndex :type Integer) (bFromSweep :type Boolean) (SweepResult :type Hit%20Result%20Structure%20%28by%20ref%29))
  ;[1 1 1] Shoot mobs in shoot zone
  (Networking|SwitchHasAuthority
    (:Authority
      (bind _asai_mob (Utilities|Casting|CastToAI_Mob OtherActor))
      (Utilities|Array|AddUnique (Variables|ServerProperties|GetTargets) _asai_mob)
      (if (== (Utilities|Array|Length (Variables|ServerProperties|GetTargets)) 1)
        (bind _returnvalue (Utilities|Time|SetTimerbyEvent (delegate Custom|Shoot) (Variables|Attributes|GetDelay) true))
        (CallFunction|IdleShotStopTimer)))))

(event OnComponentEndOverlap(TowerDamager)
  (params (OverlappedComponent :type Primitive%20Component%20Object%20Reference) (OtherActor :type Actor%20Object%20Reference) (OtherComp :type Primitive%20Component%20Object%20Reference) (OtherBodyIndex :type Integer))
  ;[1 1 1] Shoot mobs in shoot zone
  (Networking|SwitchHasAuthority
    (:Authority
      (bind _asai_mob (Utilities|Casting|CastToAI_Mob OtherActor))
      (Utilities|Array|RemoveItem (Variables|ServerProperties|GetTargets) _asai_mob)
      (if (== (Utilities|Array|Length (Variables|ServerProperties|GetTargets)) 0)
        (Utilities|Time|ClearandInvalidateTimerbyHandle (stale OnComponentBeginOverlap(TowerDamager) _returnvalue))
        (CallFunction|IdleShotStartTimer)))))

(event OnClicked(Tower)
  (params (TouchedComponent :type Primitive%20Component%20Object%20Reference) (ButtonPressed :type Key%20Structure))
  ;[1 1 1] Display Damage Status
  (bind _asbp_player_character (Utilities|Casting|CastToBP_PlayerCharacter (Game|GetPlayerCharacter 0)))
  (Default|ShowTowerStatus _asbp_player_character self))

(event Custom|UpdateTextEffect-All
  (params (Effect_WB :type E_Effects%20Enum :default "NewEnumerator0") (Text :type Text) (Remove :type Boolean))
  ;[1 1 1] EditTextEffectAll
  (Utilities|IsValid (Utilities|Select :Index Effect_WB :NewEnumerator0 0 :NewEnumerator1 0 :NewEnumerator2 (Variables|Temp|GetAccelerateEffect_WB) :NewEnumerator3 (Variables|Temp|GetIdleShotDmgEffect_WB)) :!label _label
    (:Is%20Valid
      (if Remove
        (Class|PanelWidget|RemoveChild (Variables|/Game/Blueprints/UI/AllLevels/WB_Tower.WB_Tower_C|GetEffects (Variables|Status|GetTowerStatus)) (Utilities|Select :Index Effect_WB :NewEnumerator0 0 :NewEnumerator1 0 :NewEnumerator2 (Variables|Temp|GetAccelerateEffect_WB) :NewEnumerator3 (Variables|Temp|GetIdleShotDmgEffect_WB)))
        (switch Utilities|FlowControl|Switch|SwitchonE_Effects Effect_WB :!label _label_2
          (:NewEnumerator2
            (Variables|Temp|SetAccelerateEffect_WB (select Remove 0 (stale _returnvalue)))
            (goto _label))
          (:NewEnumerator3
            (Variables|Temp|SetIdleShotDmgEffect_WB (select Remove 0 (stale _returnvalue)))
            (goto _label)))
        (else
          (Rendering|Components|TextRender|SetText (Variables|/Game/Blueprints/UI/AllLevels/WB_EffectElement.WB_EffectElement_C|GetText (Utilities|Select :Index Effect_WB :NewEnumerator0 0 :NewEnumerator1 0 :NewEnumerator2 (Variables|Temp|GetAccelerateEffect_WB) :NewEnumerator3 (Variables|Temp|GetIdleShotDmgEffect_WB))) Text))))
    (:Is%20Not%20Valid
      (if (not Remove)
        (bind _returnvalue (UserInterface|CreateWidget "/Game/Blueprints/UI/AllLevels/WB_EffectElement.WB_EffectElement_C" (Game|GetPlayerController 0) (Utilities|Struct|MakeSlateBrush "(X=72.000000,Y=72.000000)" "(Left=0.000000,Top=0.000000,Right=0.000000,Bottom=0.000000)" "(SpecifiedColor=(R=1.000000,G=1.000000,B=1.000000,A=1.000000),ColorUseRule=UseColor_Specified)" (Utilities|Select :Index Effect_WB :NewEnumerator0 0 :NewEnumerator1 0 :NewEnumerator2 "/Game/Assets/Textures/Effects/T_Accelerate.T_Accelerate" :NewEnumerator3 "/Game/Assets/Textures/Effects/T_IdleShotDmg.T_IdleShotDmg") "Image" "NoTile" "NoMirror")))
        (Widget|Panel|AddChild (Variables|/Game/Blueprints/UI/AllLevels/WB_Tower.WB_Tower_C|GetEffects (Variables|Status|GetTowerStatus)) _returnvalue)
        (goto _label_2)))))

(event Custom|TargetDeath
  (params (Mob :type AI%20Mob%20Object%20Reference))
  ;[1 1 1] Shoot mobs in shoot zone
  (Utilities|Array|RemoveItem (Variables|ServerProperties|GetTargets) Mob)
  (if (== (Utilities|Array|Length (Variables|ServerProperties|GetTargets)) 0)
    (Utilities|Time|ClearandInvalidateTimerbyHandle (stale OnComponentBeginOverlap(TowerDamager) _returnvalue))
    (CallFunction|IdleShotStartTimer)))

(event Custom|DamageApplied
  (params (Damage :type Float%20%28single-precision%29))
  ;[1 1 1] TowerDamageAppliedEvent
  (CallFunction|Add&SortTowersDPSArray Damage))

(event Custom|InitStatusMenu-Server
  ;[1 1 1] InitStatusMenuAllPlayers
  (CallFunction|InitStatusMenu self))

(event Custom|Shoot
  (bind _targets (Variables|ServerProperties|GetTargets))
  (bind _damage (Variables|Attributes|GetDamage))
  ;[1 1 1] Shoot mobs in shoot zone
  (for _index (range 0 (- (Math|Integer|Clamp(Integer) (Variables|Attributes|GetMultiShotCountOfTargets) 1 (Utilities|Array|Length _targets)) 1))
    (bind _returnvalue (CallFunction|GetBulletSpawnTransform))
    (CallFunction|SpawnBullet-All (Math|Transform|MakeTransform (.location _returnvalue) "0, 0, 0" "1,1,1") (Utilities|Array|Get(acopy) _targets _index) self (Variables|Attributes|GetBulletAnimationType) (Variables|Attributes|GetIsAutoRetarget) (Variables|Attributes|GetSlowAlpha) (Variables|Attributes|GetSlowTime) (Variables|Attributes|GetHasSlowEffect?) (Variables|Attributes|GetHasExplosionEffect?) (Variables|Attributes|GetExplosionRadius) (Variables|Attributes|GetExplosionAlpha) (Variables|Attributes|GetHasBackTimeEffect?) (Variables|Attributes|GetBackTime) (Variables|Attributes|GetHasBouncingEffect?) (Variables|Attributes|GetBouncingRadius) (Variables|Attributes|GetBouncingAlpha) (Variables|Attributes|GetBouncingCounter) (select (Variables|Attributes|GetHasIdleShotEffect?) (+ _damage (Variables|Temp|GetIdleShotAddDamage)) _damage) (Variables|Attributes|GetHasExtraDmgLone?) (Variables|Attributes|GetExtraDmgLoneRadius) (Variables|Attributes|GetExtraDmgLoneAlpha) false))
  (Variables|Temp|SetIdleShotAddDamage 0.0)
  (CallFunction|UpdateTextEffect-All "NewEnumerator3" "" true))

(event Custom|SpawnBullet-All
  (params (SpawnTransform_Location :type Transform) (Target :type AI%20Mob%20Object%20Reference) (Damager :type BP%20Tower%20Object%20Reference) (BulletAnimationType :type E_BulletAnimationType%20Enum :default "NewEnumerator0") (IsAutoTarget :type Boolean) (SlowAlpha :type Float%20%28single-precision%29) (SlowTime :type Float%20%28single-precision%29) (HasSlowEffect? :type Boolean) (HasExplosionEffect? :type Boolean) (ExplosionRadius :type Integer) (ExplosionAlpha :type Float%20%28single-precision%29) (HasBackTimeEffect? :type Boolean) (BackTime :type Float%20%28single-precision%29) (HasBouncingEffect? :type Boolean) (BouncingRadius :type Integer) (BouncingAlpha :type Float%20%28single-precision%29) (BouncingCounter :type Integer) (Damage :type Float%20%28single-precision%29) (HasExtraDmgLone? :type Boolean) (ExtraDmgLoneRadius :type Integer) (ExtraDmgLoneAlpha :type Float%20%28single-precision%29) (AnotherSource? :type Boolean) (AnotherSource :type Mesh%20Component%20Object%20Reference))
  (Utilities|SpawnBullet (.location SpawnTransform_Location) Target Damager BulletAnimationType IsAutoTarget SlowAlpha SlowTime HasSlowEffect? HasExplosionEffect? ExplosionRadius ExplosionAlpha HasBackTimeEffect? BackTime HasBouncingEffect? BouncingRadius BouncingAlpha BouncingCounter Damage HasExtraDmgLone? ExtraDmgLoneRadius ExtraDmgLoneAlpha AnotherSource? AnotherSource))

(event Custom|InitStatusMenu
  (params (Tower :type BP%20Tower%20Object%20Reference))
  ;[1 1 1] InitStatusMenuAllPlayers
  (Utilities|InitStatusMenuMacro Tower))

(event Custom|OnComponentBeginOverlap_SpeedAura
  (params (OverlappedComponent :type Primitive%20Component%20Object%20Reference) (OtherActor :type Actor%20Object%20Reference) (OtherComp :type Primitive%20Component%20Object%20Reference) (OtherBodyIndex :type Integer) (bFromSweep :type Boolean) (SweepResult :type Hit%20Result%20Structure%20%28by%20ref%29))
  ;[1 1 1] SpeedAura
  (Networking|SwitchHasAuthority
    (:Authority
      (bind _tower (Utilities|HandleOverlapforAuraActor OtherActor)
        (:Found
          (Utilities|IsValid _tower
            (:Is%20Valid
              (CallFunction|SetSpeedAura _tower (Variables|Attributes|GetSpeedAuraAlpha)))))))))

(event Custom|IdleShotAdder
  (bind _idleshotmaxdmg (Variables|Attributes|GetIdleShotMaxDmg))
  ;[1 1 1] IdleShotTimerManager
  (bind _output_get (Variables|Temp|SetIdleShotAddDamage (Math|Float|Min(Float) (+ (Variables|Temp|GetIdleShotAddDamage) (Variables|Attributes|GetIdleShotDamage)) _idleshotmaxdmg)))
  (if (== _output_get _idleshotmaxdmg)
    (CallFunction|IdleShotStopTimer))
  (CallFunction|UpdateTextEffect-All "NewEnumerator3" (Utilities|Text|ToText(Float) (/ (Math|Conversions|ToFloat(Integer) (Math|Float|Truncate (* 10 _output_get))) 1e+01) "HalfToEven") false))

(event Custom|OnComponentEndOverlap_SpeedAura
  (params (OverlappedComponent :type Primitive%20Component%20Object%20Reference) (OtherActor :type Actor%20Object%20Reference) (OtherComp :type Primitive%20Component%20Object%20Reference) (OtherBodyIndex :type Integer))
  ;[1 1 1] SpeedAura
  (Networking|SwitchHasAuthority
    (:Authority
      (bind _asbp_tower (Utilities|Casting|CastToBP_Tower OtherActor))
      (if (Utilities|Set|Contains (Variables|Temp|GetSetSpeedAuraTowers) _asbp_tower)
        (Utilities|Set|Remove (Variables|Temp|GetSetSpeedAuraTowers) _asbp_tower)
        (CallFunction|ResetSpeedAura _asbp_tower (Variables|Attributes|GetSpeedAuraAlpha))))))

(event Custom|SetSpeedAura
  (params (AccelerateAlpha :type Float%20%28single-precision%29))
  ;[1 1 1] SpeedAura
  (Variables|Attributes|SetDelay (* AccelerateAlpha (Variables|Attributes|GetDelay)))
  (CallFunction|UpdateTextEffect-All "NewEnumerator2" (Utilities|Text|ToText(Integer) (Math|Float|Truncate (/ (Math|Conversions|ToFloat(Integer) (Math|Float|Floor (/ (* 1000 (Variables|Temp|GetOriginDelayStore)) (Variables|Attributes|GetDelay)))) 1e+01))) false))

(event Custom|ResetSpeedAura
  (params (AcclerateAlpha :type Float%20%28single-precision%29))
  ;[1 1 1] SpeedAura
  (bind _output_get (Variables|Attributes|SetDelay (/ (Variables|Attributes|GetDelay) AcclerateAlpha)))
  (CallFunction|UpdateTextEffect-All "NewEnumerator2" (Utilities|Text|ToText(Integer) (Math|Float|Truncate (/ (Math|Conversions|ToFloat(Integer) (Math|Float|Floor (/ (* 1000 (Variables|Temp|GetOriginDelayStore)) (Variables|Attributes|GetDelay)))) 1e+01))) (== _output_get (Variables|Temp|GetOriginDelayStore))))

(event Custom|IdleShotStartTimer
  ;[1 1 1] IdleShotTimerManager
  (if (Variables|Attributes|GetHasIdleShotEffect?)
    (bind _returnvalue (Utilities|Time|SetTimerbyEvent (delegate Custom|IdleShotAdder) (Variables|Attributes|GetIdleShotDelay) true))
    (Variables|ServerProperties|SetIdleShotTimer _returnvalue)))

(event Custom|IdleShotStopTimer
  ;[1 1 1] IdleShotTimerManager
  (if (Variables|Attributes|GetHasIdleShotEffect?)
    (Utilities|Time|ClearandInvalidateTimerbyHandle (Variables|ServerProperties|GetIdleShotTimer))))

(event EventDestroyed
  ;[1 1 1] DestroyAnimation
  (Utilities|FlowControl|Sequence
    (:then_0
      (Effects|SpawnEmitteratLocation "/Game/StarterContent/Particles/P_Explosion.P_Explosion" (Transformation|GetActorLocation) "0, 0, 0" "2.000000,2.000000,2.000000")
      (bind _asbp_player_character (Utilities|Casting|CastToBP_PlayerCharacter (Game|GetPlayerCharacter 0)))
      (if (Utilities|Array|ContainsItem (Variables|/Game/Blueprints/Player/BP_PlayerCharacter.BP_PlayerCharacter_C|GetTowersSelected _asbp_player_character) self)
        (Default|ClearTowersStatus _asbp_player_character)))
    (:then_1
      (Utilities|IsValid (Variables|Default|GetGameInstanceRef)
        (:Is%20Valid
          (Networking|SwitchHasAuthority))))))

(event EventBeginPlay
  ;[1 1 1] Init
  (Networking|SwitchHasAuthority
    (:Authority
      (CallFunction|InitStatusMenu self))
    (:Remote
      (CallFunction|InitStatusMenu-Server)))
  (bind _asbp_game_mode (Utilities|Casting|CastToBP_GameMode (Game|GetGameMode)))
  (Variables|Default|SetGameModeRef _asbp_game_mode)
  (bind _asgi_info (Utilities|Casting|CastToGI_Info (Game|GetGameInstance)))
  (Variables|Default|SetGameInstanceRef _asgi_info)
  (bind _radiusresult (CallFunction|CellstoDistance (Variables|Attributes|GetRadius)))
  (Components|Sphere|SetSphereRadius (Variables|Default|GetTowerDamager) _radiusresult false)
  (|InitSpeedAura (Variables|Attributes|GetAuraRadius) (delegate Custom|OnComponentBeginOverlap_SpeedAura) (delegate Custom|OnComponentEndOverlap_SpeedAura)))

(event EventTick
  (params (DeltaSeconds :type Float%20%28single-precision%29))
  ;[1 1 1] EveryTicksActions
  (CallFunction|RotateStatusMenuforPlayers DeltaSeconds))

(fn ConstructionScript
  (bind _radiusresult (CallFunction|CellstoDistance (Variables|Attributes|GetRadius)))
  (Components|Sphere|SetSphereRadius (Variables|Default|GetTowerDamager) _radiusresult false))

(fn RotateStatusMenuforPlayers
  (params (DeltaTime :type Float%20%28single-precision%29))
  (bind _returnvalue (Game|GetPlayerCharacter 0))
  (bind _statusmenu (Variables|Default|GetStatusMenu))
  (bind _asbp_player_character (Utilities|Casting|CastToBP_PlayerCharacter _returnvalue))
  (Transformation|SetWorldRotation _statusmenu (Class|KismetMathLibrary|RInterptoConstant (Transformation|GetWorldRotation _statusmenu) (Math|Rotator|FindLookatRotation (Transformation|GetWorldLocation _statusmenu) (Transformation|GetWorldLocation (select (Variables|/Game/Blueprints/Player/BP_PlayerCharacter.BP_PlayerCharacter_C|GetIsCameraView _asbp_player_character) (Variables|/Script/Engine.CameraActor|GetCameraComponent (Variables|/Game/Blueprints/Player/BP_PlayerCharacter.BP_PlayerCharacter_C|GetCameraUp _asbp_player_character)) (Variables|/Script/Engine.Character|GetCapsuleComponent _returnvalue)))) DeltaTime 2.5e+02) false false))

(fn CellstoDistance
  (params (Radius :type Integer))
  (return (+ 1e+02 (Math|Conversions|ToFloat(Integer) (* 200 Radius)))))

(fn GetBulletSpawnTransform
  (return (Math|Conversions|ToTransform(Vector) (+ (Transformation|GetWorldLocation (Variables|Default|GetTower)) "0, 0,140.000000"))))

(fn Add&SortTowersDPSArray
  (params (Damage :type Float%20%28single-precision%29))
  (bind _self self)
  (bind _gameinstanceref (Variables|Default|GetGameInstanceRef))
  (bind _towerdps_tower (Variables|/Game/Blueprints/AllLevels/GI_Info.GI_Info_C|GetTowerDPS_Tower _gameinstanceref))
  (bind _towerdps_value (Variables|/Game/Blueprints/AllLevels/GI_Info.GI_Info_C|GetTowerDPS_Value _gameinstanceref))
  (bind _returnvalue (Utilities|Array|FindItem _towerdps_tower _self))
  (bind _returnvalue_2 (!= _returnvalue -1))
  (if (== (Variables|/Game/Blueprints/AllLevels/GI_Info.GI_Info_C|GetTowerDPS_TotalDamage _gameinstanceref) 0.0)
    (Utilities|Array|Add _towerdps_tower self)
    (Utilities|Array|Add _towerdps_value 1.0)
    (Variables|/Game/Blueprints/AllLevels/GI_Info.GI_Info_C|SetTowerDPS_TotalDamage _gameinstanceref (+ (Variables|/Game/Blueprints/AllLevels/GI_Info.GI_Info_C|GetTowerDPS_TotalDamage _gameinstanceref) Damage))
    (else
      (bind _new (CallFunction|CalcNewDPS (select _returnvalue_2 (Utilities|Array|Get(acopy) _towerdps_value _returnvalue) 0.0) Damage (Variables|/Game/Blueprints/AllLevels/GI_Info.GI_Info_C|GetTowerDPS_TotalDamage _gameinstanceref) true))
      (if _returnvalue_2
        (Utilities|Array|RemoveIndex _towerdps_value _returnvalue)
        (Utilities|Array|RemoveIndex _towerdps_tower _returnvalue))
      (for _index (range 0 (Utilities|Array|LastIndex _towerdps_value))
        (bind _new_2 (CallFunction|CalcNewDPS (Utilities|Array|Get(acopy) _towerdps_value _index) Damage (Variables|/Game/Blueprints/AllLevels/GI_Info.GI_Info_C|GetTowerDPS_TotalDamage _gameinstanceref) false))
        (Utilities|Array|SetArrayElem _towerdps_value _index _new_2)
        (if (and (not (LocalVariables|GetAdded)) (> _new (Utilities|Array|Get(acopy) _towerdps_value _index)))
          (Utilities|Array|Insert _towerdps_tower self _index)
          (Utilities|Array|Insert _towerdps_value _new _index)
          (Variables|/Game/Blueprints/AllLevels/GI_Info.GI_Info_C|SetTowerDPS_TotalDamage _gameinstanceref (+ (Variables|/Game/Blueprints/AllLevels/GI_Info.GI_Info_C|GetTowerDPS_TotalDamage _gameinstanceref) Damage))
          (LocalVariables|SetAdded true)
          (Math|Integer|IncrementInt _index)))
      (if (LocalVariables|GetAdded)
        _
        (else
          (Utilities|Array|Add _towerdps_value _new)
          (Utilities|Array|Add _towerdps_tower self)
          (Variables|/Game/Blueprints/AllLevels/GI_Info.GI_Info_C|SetTowerDPS_TotalDamage _gameinstanceref (+ (Variables|/Game/Blueprints/AllLevels/GI_Info.GI_Info_C|GetTowerDPS_TotalDamage _gameinstanceref) Damage))))))
  (return))

(fn CalcNewDPS
  (params (Old :type Float%20%28single-precision%29) (Damage :type Float%20%28single-precision%29) (TotalDamage :type Float%20%28single-precision%29) (DamageApplied :type Boolean))
  (bind _returnvalue (/ Damage TotalDamage))
  (return (/ (select DamageApplied (+ Old _returnvalue) Old) (+ _returnvalue 1.0))))