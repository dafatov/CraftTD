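; BP_Cell is a map cell that handles cursor hover and clicks, forwarding them to BP_PlayerCharacter.
; On BeginPlay it flags itself as a core cell if any BP_Spawner's PathTargets contains its location.
; Hovering selects and highlights it until cursor exit or a time-dilation-scaled delay, while a looping timer restores gold material when unselected.
; Clicks trigger the player's Action using GI_Info's current ActionMode, except in one mode.
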(event OnBeginCursorOver(Plate)
  (params (TouchedComponent :type Primitive%20Component%20Object%20Reference))
  (bind _self self)
  ;[1 1 1] Run events to highlighted this cell if cursor over
  (bind _asbp_player_character (Utilities|Casting|CastToBP_PlayerCharacter (Game|GetPlayerCharacter 0)))
  (Variables|/Game/Blueprints/Player/BP_PlayerCharacter.BP_PlayerCharacter_C|SetSelectedCell _asbp_player_character _self)
  (Default|HighlightedCell _asbp_player_character _self)
  (Utilities|FlowControl|RetriggerableDelay (* (Class|GameplayStatics|GetGlobalTimeDilation) 0.333333))
  (Default|UnhighlightedCell _asbp_player_character _self false))

(event OnEndCursorOver(Plate)
  (params (TouchedComponent :type Primitive%20Component%20Object%20Reference))
  ;[1 1 1] Run events to highlighted this cell if cursor over
  (bind _asbp_player_character (Utilities|Casting|CastToBP_PlayerCharacter (Game|GetPlayerCharacter 0)))
  (Default|UnhighlightedCell _asbp_player_character self true))

(event OnClicked(Plate)
  (params (TouchedComponent :type Primitive%20Component%20Object%20Reference) (ButtonPressed :type Key%20Structure))
  (bind _gameinstanceref (Variables|ServerProperties|GetGameInstanceRef))
  (bind _actionmode (Variables|/Game/Blueprints/AllLevels/GI_Info.GI_Info_C|GetActionMode _gameinstanceref))
  (Utilities|IsValid _gameinstanceref
    (:Is%20Valid
      (bind _asbp_player_character (Utilities|Casting|CastToBP_PlayerCharacter (Game|GetPlayerCharacter 0)))
      (if (Utilities|Enum|NotEqual(Enum) _actionmode "NewEnumerator0")
        (Default|Action _asbp_player_character self _actionmode)))))

(event Custom|ClearSelected
  (bind _asbp_player_character (Utilities|Casting|CastToBP_PlayerCharacter (Game|GetPlayerCharacter 0)))
  (if (not (== (Variables|/Game/Blueprints/Player/BP_PlayerCharacter.BP_PlayerCharacter_C|GetSelectedCell _asbp_player_character) self))
    (Rendering|Material|SetMaterial (Variables|Default|GetPlate) 0 "/Game/StarterContent/Materials/M_Metal_Gold.M_Metal_Gold")))

(event EventBeginPlay
  (bind _self self)
  (bind _defaultsceneroot (Variables|Default|GetDefaultSceneRoot _self))
  (bind _returnvalue (Transformation|GetWorldLocation _defaultsceneroot))
  (bind _asgi_info (Utilities|Casting|CastToGI_Info (Game|GetGameInstance)))
  (Variables|ServerProperties|SetGameInstanceRef _asgi_info)
  (bind _iscore_ (CallFunction|GetIsCoreCellGlobal (Math|Vector|MakeVector (.x _returnvalue) (.y _returnvalue) 5e+01)))
  (Variables|ServerProperties|SetIsCoreCell? _iscore_)
  (Utilities|Time|SetTimerbyEvent (delegate Custom|ClearSelected) 3.0 true))

(fn ConstructionScript)

(fn GetIsCoreCellGlobal
  (params (WorldLocation :type Vector%20%28by%20ref%29))
  (bind _outactors (Actor|GetAllActorsOfClass "/Game/Blueprints/Map/BP_Spawner.BP_Spawner_C"))
  (bind _array_element (Utilities|Array|ForEachLoopwithBreak _outactors :!label _label)
    (:LoopBody
      (if (Utilities|Array|ContainsItem (Variables|/Game/Blueprints/Map/BP_Spawner.BP_Spawner_C|GetPathTargets _array_element) WorldLocation)
        (bind _output_get (LocalVariables|SetIsCoreGlobal? true))
        (goto _label Break)))
    (:Completed
      (return _output_get))))