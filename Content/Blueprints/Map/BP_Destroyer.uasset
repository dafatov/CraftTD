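; End-of-path actor that tracks the player base's health and removes AI mobs that reach it, with overlap logic running on authority only.
; The Finish volume makes arriving mobs immortal.
; DeathCollision destroys mobs, with living ones first subtracting their health as a percentage of WaveHealthGlobal from base health.
; When base health, rounded to two decimals, hits zero, it calls GameFinishDisableAndAnnounce(false) on player character 0.
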(event OnComponentBeginOverlap(Finish)
  (params (OverlappedComponent :type Primitive%20Component%20Object%20Reference) (OtherActor :type Actor%20Object%20Reference) (OtherComp :type Primitive%20Component%20Object%20Reference) (OtherBodyIndex :type Integer) (bFromSweep :type Boolean) (SweepResult :type Hit%20Result%20Structure%20%28by%20ref%29))
  ;[1 1 1] Damage Player's Base
  (Networking|SwitchHasAuthority
    (:Authority
      (bind _asai_mob (Utilities|Casting|CastToAI_Mob OtherActor))
      (Variables|/Game/Blueprints/AI/Mobs/AI_Mob.AI_Mob_C|SetIsImmortal _asai_mob true))))

(event OnComponentBeginOverlap(DeathCollision)
  (params (OverlappedComponent :type Primitive%20Component%20Object%20Reference) (OtherActor :type Actor%20Object%20Reference) (OtherComp :type Primitive%20Component%20Object%20Reference) (OtherBodyIndex :type Integer) (bFromSweep :type Boolean) (SweepResult :type Hit%20Result%20Structure%20%28by%20ref%29))
  ;[1 1 1] Damage Player's Base
  (Networking|SwitchHasAuthority
    (:Authority
      (bind _asai_mob (Utilities|Casting|CastToAI_Mob OtherActor))
      (if (Variables|/Game/Blueprints/AI/Mobs/AI_Mob.AI_Mob_C|GetisDead _asai_mob)
        _
        (else
          (bind _output_get (Variables|ServerAttributes|SetCurrentBaseHealth (- (Variables|ServerAttributes|GetCurrentBaseHealth) (/ (* 100 (Variables|/Game/Blueprints/AI/Mobs/AI_Mob.AI_Mob_C|GetHealth _asai_mob)) (Variables|Default|GetWaveHealthGlobal)))))
          (bind _result (CallFunction|RoundSpecific _output_get 2))
          (if (<= _result 0.0)
            (bind _asbp_player_character (Utilities|Casting|CastToBP_PlayerCharacter (Game|GetPlayerCharacter 0)))
            (Default|GameFinish:DisableandAnnounce _asbp_player_character false))))
      (Actor|DestroyActor _asai_mob))))

(event EventBeginPlay
  (Variables|ServerAttributes|SetCurrentBaseHealth (Variables|ServerAttributes|GetMaxBaseHealth)))

(fn ConstructionScript)

(fn RoundSpecific
  (params (Value :type Float%20%28single-precision%29) (AfterPoint :type Integer))
  (bind _returnvalue (Math|Conversions|ToFloat(Integer) AfterPoint))
  (bind _returnvalue_2 (Math|Float|Power 1e+01 _returnvalue))
  (return (/ (Math|Conversions|ToFloat(Integer) (Math|Float|Round (* Value _returnvalue_2))) _returnvalue_2)))